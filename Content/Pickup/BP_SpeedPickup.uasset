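; BP_SpeedPickup is a pickup that permanently raises the ship's speed when collected.
; When its Shield component overlaps a BP_Ship, it adds a fixed amount to that ship's Speed variable.
; It then shows a Mongolian "speed increased" notification with the new value and destroys itself.
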(event OnComponentBeginOverlap(Shield)
  (params (OverlappedComponent :type Primitive%20Component%20Object%20Reference) (OtherActor :type Actor%20Object%20Reference) (OtherComp :type Primitive%20Component%20Object%20Reference) (OtherBodyIndex :type Integer) (bFromSweep :type Boolean) (SweepResult :type Hit%20Result%20Structure%20%28by%20ref%29))
  (bind _asbp_ship (Utilities|Casting|CastToBP_Ship OtherActor))
  (bind _output_get (Variables|/Game/Character/Ship/Ship/BP_Ship.BP_Ship_C|SetSpeed _asbp_ship (+ (Variables|/Game/Character/Ship/Ship/BP_Ship.BP_Ship_C|GetSpeed _asbp_ship) 1e+02)))
  (CallFunction|CreateNotification (Utilities|Text|ToText(String) (Utilities|String|Append "Хурд ихэслээ: " (Utilities|String|ToString(Float) _output_get))))
  (Actor|DestroyActor))

(event EventBeginPlay)

(event Collision|EventActorBeginOverlap
  (params (OtherActor :type Actor%20Object%20Reference)))

(event EventTick
  (params (DeltaSeconds :type Float%20%28single-precision%29))
  (|CallParentFunction DeltaSeconds) ; This node is disabled and will not be called.\nDrag off pins to build functionality.
)

(fn ConstructionScript
  (|CallParentFunction))