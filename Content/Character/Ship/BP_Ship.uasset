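; BP_Ship is the player's ship, with twin blasters, health and a scripted launch.
; Each tick it first follows a start spline while steering control rotation, then after a few seconds flies forward along that rotation.
; Each blaster spawns beams with its own time-based cooldown.
; Debris hits shake the camera, reduce health on the orientation screen and, at zero, trigger game over, an explosion and destruction of ship, Kinect character, screen and wheel.
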(event Custom|onDebrisHit
  (params (Damage :type Float%20%28single-precision%29))
  (bind _orientationscreen (Variables|Default|GetOrientationScreen))
  ;[0 0 0] Collision Function
  (Camera|PlayWorldCameraShake "/Game/Obstacle/Debris/BP_DebrisShake.BP_DebrisShake_C" (Transformation|GetActorLocation) 0.0 5e+02)
  (bind _output_get (Variables|Default|SetHealthPoints (- (Variables|Default|GetHealthPoints) Damage)))
  (Utilities|IsValid _orientationscreen
    (:Is%20Valid
      (Default|ChangeHealth _orientationscreen (Math|Float|Truncate _output_get)))
    (:Is%20Not%20Valid
      _))
  (CallFunction|CheckGameOver))

(event Custom|ShootLeftBeam
  (bind _leftblaster (Variables|Default|GetLeftBlaster))
  ;[0 0 0] Blasters
  (if (< (+ (Variables|Default|GetLastLeftBeam) (Math|Timespan|MakeTimespan 0 0 0 0 200)) (Math|DateTime|Now))
    (Variables|Default|SetLastLeftBeam (Math|DateTime|Now))
    (Game|SpawnActorfromClass "/Game/Character/Ship/BP_BlasterBeam.BP_BlasterBeam_C" (Math|Transform|MakeTransform (Transformation|GetWorldLocation _leftblaster) (Transformation|GetWorldRotation _leftblaster) "1,1,1") "Undefined" 0 self 0)))

(event Custom|ShootRightBeam
  (bind _returnvalue (Math|DateTime|Now))
  (bind _rightblaster (Variables|Default|GetRightBlaster))
  ;[0 0 0] Blasters
  (if (< (+ (Variables|Default|GetLastRightBeam) (Math|Timespan|MakeTimespan 0 0 0 0 200)) _returnvalue)
    (Variables|Default|SetLastRightBeam _returnvalue)
    (Game|SpawnActorfromClass "/Game/Character/Ship/BP_BlasterBeam.BP_BlasterBeam_C" (Math|Transform|MakeTransform (Transformation|GetWorldLocation _rightblaster) (Transformation|GetWorldRotation _rightblaster) "1,1,1") "Undefined" 0 self 0)))

(event EventTick
  (params (DeltaSeconds :type Float%20%28single-precision%29))
  ;[0 0 0] Tick
  (CallFunction|MoveStart DeltaSeconds)
  (CallFunction|MoveForward))

(fn ConstructionScript)

(fn MoveForward
  (bind _returnvalue (Pawn|GetControlRotation :!class /Script/Engine.Pawn))
  (if (Variables|Default|GetisStarted)
    (Transformation|AddActorWorldOffset (* (Math|Vector|GetForwardVector (Math|Rotator|MakeRotator (.roll _returnvalue) (.pitch _returnvalue) (.yaw _returnvalue))) (Variables|Default|GetActualSpeed)))))

(fn MoveStart
  (params (DeltaSeconds :type Float%20%28single-precision%29))
  (if (not (Variables|Default|GetisStarted))
    (Variables|Default|SetSeconds (+ DeltaSeconds (Variables|Default|GetSeconds)))
    (Transformation|SetActorLocation (.location (Spline|GetTransformatDistanceAlongSpline (Variables|/Game/Menu/MenuShip/BP_Spline.BP_Spline_C|GetSpline (Variables|Default|GetStartSpline)) (* (Variables|Default|GetSeconds) (Variables|Default|GetStartSpeed)) "World" false)) false false)
    (Pawn|SetControlRotation (Pawn|GetController) (.rotation (Spline|GetTransformatDistanceAlongSpline (Variables|/Game/Menu/MenuShip/BP_Spline.BP_Spline_C|GetSpline (Variables|Default|GetStartSpline)) (* (Variables|Default|GetSeconds) (Variables|Default|GetStartSpeed)) "World" false)))
    (if (> (Variables|Default|GetSeconds) 3.6)
      (Variables|Default|SetisStarted true))))

(fn CheckGameOver
  (if (<= (Variables|Default|GetHealthPoints) 0.0)
    (bind _returnvalue (UserInterface|CreateWidget "/Game/Menu/PauseMenu/W_GameOver.W_GameOver_C" (Game|GetPlayerController 0)))
    (UserInterface|Viewport|AddtoViewport _returnvalue 0)
    (Effects|SpawnEmitteratLocation "/Game/StarterContent/Particles/P_Explosion.P_Explosion" "0, 0, 0")
    (Actor|DestroyActor (Variables|Default|GetKinectCharacter))
    (Default|CustomDestroy (Variables|Default|GetOrientationScreen))
    (Actor|DestroyActor (Variables|Default|GetWheel))
    (Actor|DestroyActor)))