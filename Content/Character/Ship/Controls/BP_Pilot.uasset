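; Ship pilot Blueprint that mirrors the player's Kinect-tracked hands onto two in-game hand meshes, with the left one flipped by negative Y scale.
; It spawns BP_KinectTracker on BeginPlay, then each tick maps hand joints, relative to a reference joint, into clamped positions, waiting for Ship.IsStarted in StartLevel.
; AnimateHands switches only the left hand between grab and open animations.
; Hand rotation functions exist but are not called here.
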(event EventTick
  (params (DeltaSeconds :type Float%20%28single-precision%29))
  (bind _returnvalue (Game|GetCurrentLevelName true))
  (if (Utilities|Enum|Equal(Enum) _returnvalue "StartLevel")
    (if (Variables|/Game/Character/Ship/Ship/BP_Ship.BP_Ship_C|GetisStarted (Variables|Default|GetShip))
      (CallFunction|MoveLeftHand :!label _label)
      (CallFunction|MoveRightHand)
      (CallFunction|AnimateHands))
    (else
      (goto _label))))

(event EventBeginPlay
  ;[0 0 0] Spawn Kinect Tracker
  (bind _returnvalue (Game|SpawnActorfromClass "/Game/Character/Tracker/BP_KinectTracker.BP_KinectTracker_C" (Transformation|GetActorTransform) "Undefined" 0 0))
  (Variables|Default|SetKinectTracker _returnvalue))

(fn ConstructionScript
  (bind _handscale (Variables|Default|GetHandScale))
  (Transformation|SetRelativeScale3D (Variables|Default|GetLeftHand) (Math|Vector|MakeVector (.x _handscale) (* -1 (.y _handscale)) (.z _handscale)))
  (Transformation|SetRelativeScale3D (Variables|Default|GetRightHand) (Variables|Default|GetHandScale)))

(fn MoveLeftHand
  (bind _relativemovement (Kinect|GetRelativeMovement "NewEnumerator7" "NewEnumerator0"))
  (Utilities|FlowControl|Sequence
    (:then_0
      ;[0 0 0] Horizontal Movement
      (LocalVariables|SetHorizontalPosition (Math|Float|Min(Float) (- 0.0 (* 30 (- 1.0 (Math|Float|Min(Float) (Math|Float|Max(Float) (Math|Float|NormalizetoRange (.x _relativemovement) -0.1 -0.6) 0.0) 1.0)))) -5.0)))
    (:then_1
      ;[0 0 0] Vertical Movement
      (LocalVariables|SetVerticalPosition (+ (* 30 (Math|Float|Min(Float) (Math|Float|Max(Float) (Math|Float|NormalizetoRange (.y _relativemovement) 0.0 1.0) 0.0) 1.0)) 15.0)))
    (:then_2
      ;[0 0 0] Set Location
      (Transformation|SetRelativeLocation (Variables|Default|GetLeftHand) (Math|Vector|MakeVector 25.0 (LocalVariables|GetHorizontalPosition) (LocalVariables|GetVerticalPosition)) false false))))

(fn MoveRightHand
  (bind _relativemovement (Kinect|GetRelativeMovement "NewEnumerator11" "NewEnumerator0"))
  (Utilities|FlowControl|Sequence
    (:then_0
      ;[0 0 0] Horizontal Movement
      (LocalVariables|SetHorizontalPosition (Math|Float|Max(Float) (+ (* 30 (Math|Float|Min(Float) (Math|Float|Max(Float) (Math|Float|NormalizetoRange (.x _relativemovement) -0.2 0.5) 0.0) 1.0)) 0.0) 5.0)))
    (:then_1
      ;[0 0 0] Vertical Movement
      (LocalVariables|SetVerticalPosition (+ (* 30 (Math|Float|Min(Float) (Math|Float|Max(Float) (Math|Float|NormalizetoRange (.y _relativemovement) 0.0 1.0) 0.0) 1.0)) 15.0)))
    (:then_2
      ;[0 0 0] Set Location
      (Transformation|SetRelativeLocation (Variables|Default|GetRightHand) (Math|Vector|MakeVector 25.0 (LocalVariables|GetHorizontalPosition) (LocalVariables|GetVerticalPosition)) false false))))

(fn RotateLeftHand
  (bind _result (Default|GetJointRotator (Variables|Default|GetKinectTracker) "NewEnumerator7"))
  (Transformation|SetRelativeRotation (Variables|Default|GetLeftHand) (Math|Rotator|MakeRotator (+ (* 90 (Math|Float|Max(Float) (Math|Float|Min(Float) (Math|Float|NormalizetoRange (.pitch _result) -5e+01 2e+01) 1.0) 0.0)) -9e+01) 0.0 0.0) true false))

(fn RotateRightHand
  (bind _result (Default|GetJointRotator (Variables|Default|GetKinectTracker) "NewEnumerator11"))
  (Transformation|SetRelativeRotation (Variables|Default|GetRightHand) (Math|Rotator|MakeRotator (+ (* 90 (- 1.0 (Math|Float|Max(Float) (Math|Float|Min(Float) (Math|Float|NormalizetoRange (.pitch _result) -5e+01 -1e+01) 1.0) 0.0))) 0.0) 0.0 0.0) true false))

(fn GetRelativeMovement
  (params (Joint :type E_JointNameEnum%20Enum :default "NewEnumerator0") (RelativeTo :type E_JointNameEnum%20Enum :default "NewEnumerator0"))
  (bind _kinecttracker (Variables|Default|GetKinectTracker))
  (bind _result (Default|GetJointVector _kinecttracker Joint))
  (bind _result_2 (Default|GetJointVector _kinecttracker RelativeTo))
  (return (- _result _result_2)))

(fn AnimateHands
  (bind _lefthand (Variables|Default|GetLeftHand))
  (bind _lefthand_2 (Variables|Default|GetLeftHand))
  (bind _returnvalue (Class|KinectActor|GetLeftHandState (Variables|Default|GetKinectTracker)))
  (if _returnvalue
    (Components|Animation|SetAnimation _lefthand_2 "/Game/Models/Mannequin/Animations/MannequinHand_Right_Grab.MannequinHand_Right_Grab")
    (Audio|Components|Audio|Play _lefthand_2 false)
    (else
      (Components|Animation|SetAnimation _lefthand "/Game/Models/Mannequin/Animations/MannequinHand_Right_Open.MannequinHand_Right_Open")
      (Audio|Components|Audio|Play _lefthand false))))