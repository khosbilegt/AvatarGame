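; Blaster beam projectile for the ship that flies straight along its spawn rotation and breaks up debris it hits.
; On BeginPlay it adds the ship's speed to its own and plays a beam sound, then Tick moves the Billboard by a per-frame step, not scaled by delta time.
; A Delay in Tick counts seconds to self-destruct.
; Box overlap with BP_Debris calls Impact, spawns a Niagara explosion and destroys the beam.
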(event OnComponentBeginOverlap(Box)
  (params (OverlappedComponent :type Primitive%20Component%20Object%20Reference) (OtherActor :type Actor%20Object%20Reference) (OtherComp :type Primitive%20Component%20Object%20Reference) (OtherBodyIndex :type Integer) (bFromSweep :type Boolean) (SweepResult :type Hit%20Result%20Structure%20%28by%20ref%29))
  (bind _box (Variables|Default|GetBox))
  (bind _returnvalue (Transformation|GetWorldLocation _box))
  (bind _asbp_debris (Utilities|Casting|CastToBP_Debris OtherActor))
  (Default|Impact _asbp_debris _returnvalue (Math|Vector|GetForwardVector _box))
  (Niagara|SpawnSystematLocation "/Game/Models/TieFighter/Particle/NS_BlastExplosion.NS_BlastExplosion" _returnvalue)
  (Actor|DestroyActor))

(event EventBeginPlay
  (Variables|Default|SetActualSpeed (+ (Variables|Default|GetSpeed) (Variables|Default|GetShipActualSpeed)))
  (Variables|Default|SetRotation (Transformation|GetActorRotation))
  (Audio|PlaySoundatLocation "/Game/Sound/MP_Beam.MP_Beam" (Transformation|GetActorLocation) "0, 0, 0" 0.5 1.0 0.0 0 0 0))

(event EventTick
  (params (DeltaSeconds :type Float%20%28single-precision%29))
  (Transformation|SetWorldLocation (Variables|Default|GetBillboard) (+ (* (Math|Vector|GetForwardVector (Variables|Default|GetRotation)) (Variables|Default|GetActualSpeed)) (Transformation|GetWorldLocation (Variables|Default|GetBillboard))) false false)
  (Utilities|FlowControl|Delay 1.0)
  (bind _result (Math|Float|IncrementFloat (Variables|Default|GetSeconds))
    (:%20%20
      (Variables|Default|SetSeconds _result)
      (if (> (Variables|Default|GetSeconds) 3.0)
        (Actor|DestroyActor)))))

(fn ConstructionScript)