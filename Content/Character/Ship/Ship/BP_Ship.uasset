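; Player-controlled spaceship that flies, fires rate-limited twin blasters and takes debris damage, with an IsModify mode that skips flight.
; Tick follows a start spline, then pushes the ship forward along control rotation.
; Zero health or the portal video triggers a self-recursive countdown that fades out to MenuLevel.
; Interior colors load from and save to JSON via VaRest and CustomFileHelper, tinting the cockpit light, back camera, GPS and radar.
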(event Custom|onDebrisHit
  (params (Damage :type Float%20%28single-precision%29))
  (bind _backcamera (Variables|Blueprints|GetBackCamera))
  (bind _radar (Variables|/Game/Character/Ship/Screens/BP_BackScreen.BP_BackScreen_C|GetRadar _backcamera))
  ;[0 0 0] Collision Function
  (Camera|PlayWorldCameraShake "/Game/Obstacle/Debris/BP_DebrisShake.BP_DebrisShake_C" (Transformation|GetActorLocation) 0.0 5e+02)
  (bind _output_get (Variables|Float|SetHealthPoints (- (Variables|Float|GetHealthPoints) Damage)))
  (Utilities|IsValid _radar
    (:Is%20Valid
      (Default|ChangeHealth _radar (Math|Float|Truncate _output_get)))
    (:Is%20Not%20Valid
      _))
  (Game|CheckGameOver))

(event Custom|ShootLeftBeam
  (bind _leftblaster (Variables|Default|GetLeftBlaster))
  ;[0 0 0] Blasters
  (if (< (+ (Variables|Default|GetLastLeftBeam) (Math|Timespan|MakeTimespan 0 0 0 0 200)) (Math|DateTime|Now))
    (Variables|Default|SetLastLeftBeam (Math|DateTime|Now))
    (Game|SpawnActorfromClass "/Game/Character/Ship/Ship/BP_BlasterBeam.BP_BlasterBeam_C" (Math|Transform|MakeTransform (Transformation|GetWorldLocation _leftblaster) (Transformation|GetWorldRotation _leftblaster) "1,1,1") "Undefined" 0 self 0)))

(event Custom|ShootRightBeam
  (bind _returnvalue (Math|DateTime|Now))
  (bind _rightblaster (Variables|Default|GetRightBlaster))
  ;[0 0 0] Blasters
  (if (< (+ (Variables|Default|GetLastRightBeam) (Math|Timespan|MakeTimespan 0 0 0 0 200)) _returnvalue)
    (Variables|Default|SetLastRightBeam _returnvalue)
    (Game|SpawnActorfromClass "/Game/Character/Ship/Ship/BP_BlasterBeam.BP_BlasterBeam_C" (Math|Transform|MakeTransform (Transformation|GetWorldLocation _rightblaster) (Transformation|GetWorldRotation _rightblaster) "1,1,1") "Undefined" 0 self 0)))

(event Custom|Play%20Portal%20Video
  ;[0 0 0] Portal Video
  (Rendering|SetVisibility (Variables|Default|GetPlane) true false)
  (Media|MediaPlayer|OpenSource (Variables|Default|GetMediaPlayer) "/Game/Obstacle/Portal/MP_Portal.MP_Portal")
  (CallFunction|ReturntoMain))

(event Custom|returnToMain
  ;[0 0 0] Game Over Function
  (Audio|Components|Audio|SetVolumeMultiplier (Variables|Default|GetEngineAudio) 0.0 :!class /Script/Engine.AudioComponent)
  (Variables|Default|SetisOver true)
  (if (== (Variables|Float|GetoverSeconds) 0.0)
    (bind _returnvalue (UserInterface|CreateWidget "/Game/Menu/EndMenu/W_EndCountdown.W_EndCountdown_C"))
    (bind _output_get (Variables|Default|SetCountdown _returnvalue))
    (UserInterface|Viewport|AddtoViewport _output_get 0)
    (Variables|Float|SetoverSeconds (+ (Variables|Float|GetoverSeconds) 1.0) :!label _label)
    (Utilities|FlowControl|Delay 1.0)
    (CallFunction|ReturntoMain)
    (elif (< (Variables|Float|GetoverSeconds) 1e+01)
      (Default|SetCount (Variables|Default|GetCountdown) (Variables|Float|GetoverSeconds) false)
      (goto _label)
      (else
        (CallFunction|OpenLevelWrapper "MenuLevel")))))

(event Custom|OpenLevelWrapper
  (params (LevelName :type Name))
  (bind _returnvalue (UserInterface|CreateWidget "/Game/Menu/EndMenu/W_FadeOut.W_FadeOut_C" 0 LevelName))
  (UserInterface|Viewport|AddtoViewport _returnvalue 0))

(event EventBeginPlay
  ;[0 0 0] Begin Play
  (if (Variables|Default|GetisModify)
    (Modify|ModifyBegin)
    (Modify|SetColors)
    (else
      (Audio|PlaySoundatLocation "/Game/Sound/MP_Start.MP_Start" (Transformation|GetActorLocation) "0, 0, 0" 1.0 1.0 0.0 0 0 0)
      (Modify|SetColors)
      (Utilities|FlowControl|Delay 3.0)
      (bind _returnvalue (Audio|SpawnSoundAttached "/Game/Sound/MP_Engine.MP_Engine" (Variables|Default|GetPlayerView) "None" "0, 0, 0" "0, 0, 0" "KeepRelativeOffset" false 1.0 1.0 0.0 0 0))
      (Variables|Default|SetEngineAudio _returnvalue))))

(event EventTick
  (params (DeltaSeconds :type Float%20%28single-precision%29))
  ;[0 0 0] Tick
  (if (not (Variables|Default|GetisModify))
    (if (not (Variables|Default|GetisOver))
      (Game|MoveStart DeltaSeconds)
      (Game|MoveForward))))

(fn ConstructionScript)

(fn ModifyBegin
  (bind _returnvalue (Rendering|Material|CreateDynamicMaterialInstance (Variables|Default|GetWindow) 0 "/Game/Menu/MenuShip/M_ShipColor.M_ShipColor" "None" :!class /Script/Engine.PrimitiveComponent))
  (Rendering|Material|SetScalarParameterValue _returnvalue "Appearance" 1.0 :!class /Script/Engine.MaterialInstanceDynamic)
  (Rendering|Material|SetVectorParameterValue _returnvalue "Color" (Utilities|Array|Get(acopy) (Variables|Modify|GetColors)) :!class /Script/Engine.MaterialInstanceDynamic)
  (Rendering|Material|SetMaterial (Variables|Default|GetWindow) 0 _returnvalue))

(fn FadeOut
  (params (deltaSeconds :type Float%20%28single-precision%29))
  (bind _returnvalue (/ deltaSeconds 3.0))
  (bind _window (Variables|Default|GetWindow))
  (bind _returnvalue_2 (+ 0.0 _returnvalue))
  (if (not (Variables|Modify|GetisFaded))
    (for (_ _array_index) (Rendering|Material|GetMaterials _window)
      (bind _returnvalue_3 (Rendering|Material|CreateDynamicMaterialInstance _window 0 "/Game/Menu/MenuShip/M_ShipColor.M_ShipColor" "None" :!class /Script/Engine.PrimitiveComponent))
      (bind _output_get (LocalVariables|SetMaterialInstance _returnvalue_3))
      (Rendering|Material|SetScalarParameterValue _output_get "Appearance" _returnvalue_2 :!class /Script/Engine.MaterialInstanceDynamic)
      (Rendering|Material|SetVectorParameterValue (LocalVariables|GetMaterialInstance) "Color" (Utilities|Array|Get(acopy) (Variables|Modify|GetColors) _array_index) :!class /Script/Engine.MaterialInstanceDynamic)
      (Rendering|Material|SetMaterial (Variables|Default|GetWindow) _array_index (LocalVariables|GetMaterialInstance))
      (if (> _returnvalue_2 1.0)
        (Variables|Modify|SetisFaded true)))))

(fn MoveForward
  (bind _returnvalue (Pawn|GetControlRotation :!class /Script/Engine.Pawn))
  (if (Variables|Default|GetisStarted)
    (Transformation|AddActorWorldOffset (* (Math|Vector|GetForwardVector (Math|Rotator|MakeRotator (.roll _returnvalue) (.pitch _returnvalue) (.yaw _returnvalue))) (Variables|Float|GetActualSpeed)))))

(fn MoveStart
  (params (DeltaSeconds :type Float%20%28single-precision%29))
  (if (not (Variables|Default|GetisStarted))
    (Variables|Float|SetSeconds (+ DeltaSeconds (Variables|Float|GetSeconds)))
    (Transformation|SetActorLocation (.location (Spline|GetTransformatDistanceAlongSpline (Variables|/Game/Menu/MenuShip/BP_Spline.BP_Spline_C|GetSpline (Variables|Blueprints|GetStartSpline)) (* (Variables|Float|GetSeconds) (Variables|Float|GetStartSpeed)) "World" false)) false false)
    (Pawn|SetControlRotation (Pawn|GetController) (.rotation (Spline|GetTransformatDistanceAlongSpline (Variables|/Game/Menu/MenuShip/BP_Spline.BP_Spline_C|GetSpline (Variables|Blueprints|GetStartSpline)) (* (Variables|Float|GetSeconds) (Variables|Float|GetStartSpeed)) "World" false)))
    (if (> (Variables|Float|GetSeconds) 3.6)
      (Variables|Default|SetisStarted true))))

(fn CheckGameOver
  (if (and (not (Variables|Default|GetisOver)) (<= (Variables|Float|GetHealthPoints) 0.0))
    (bind _returnvalue (UserInterface|CreateWidget "/Game/Menu/EndMenu/W_GameOver.W_GameOver_C" (Game|GetPlayerController 0)))
    (UserInterface|Viewport|AddtoViewport _returnvalue 0)
    (Effects|SpawnEmitteratLocation "/Game/StarterContent/Particles/P_Explosion.P_Explosion" "0, 0, 0")
    (Actor|DestroyActor (Variables|Kinect|GetKinectCharacter))
    (Default|CustomDestroy (Variables|Blueprints|GetBackCamera))
    (Actor|DestroyActor (Variables|Blueprints|GetWheel))
    (Rendering|SetVisibility (Variables|Default|GetPlayerView) false false)
    (Audio|PlaySoundatLocation "/Game/Sound/MP_Explosion.MP_Explosion" "0, 0, 0" "0, 0, 0" 1.0 1.0 1.0 0 0 0)
    (CallFunction|ReturntoMain)))

(fn Fadein
  (params (deltaSeconds :type Float%20%28single-precision%29))
  (bind _returnvalue (/ deltaSeconds 3.0))
  (bind _window (Variables|Default|GetWindow))
  (bind _returnvalue_2 (- 1.0 _returnvalue))
  (if (not (Variables|Modify|GetisFaded))
    (for (_ _array_index) (Rendering|Material|GetMaterials _window)
      (bind _returnvalue_3 (Rendering|Material|CreateDynamicMaterialInstance _window 0 "/Game/Menu/MenuShip/M_ShipColor.M_ShipColor" "None" :!class /Script/Engine.PrimitiveComponent))
      (bind _output_get (LocalVariables|SetMaterialInstance _returnvalue_3))
      (Rendering|Material|SetScalarParameterValue _output_get "Appearance" _returnvalue_2 :!class /Script/Engine.MaterialInstanceDynamic)
      (Rendering|Material|SetVectorParameterValue (LocalVariables|GetMaterialInstance) "Color" (Utilities|Array|Get(acopy) (Variables|Modify|GetColors) _array_index) :!class /Script/Engine.MaterialInstanceDynamic)
      (Rendering|Material|SetMaterial (Variables|Default|GetWindow) _array_index (LocalVariables|GetMaterialInstance))
      (if (< _returnvalue_2 0.0)
        (Variables|Modify|SetisFaded true)))))

(fn SetColors
  (bind _backcamera (Variables|Blueprints|GetBackCamera))
  (Utilities|FlowControl|Sequence
    (:then_0
      ;[0 0 0] Handles JSON
      (bind _returnvalue (Game|SpawnActorfromClass "/Script/CombatGame.CustomFileHelper" (Transformation|GetActorTransform) "Undefined" 0 0))
      (bind _returnvalue_2 (Class|CustomFileHelper|LoadFile _returnvalue "interior_colors.json"))
      (bind _returnvalue_3 (Class|VaRestSubsystem|DecodeJsonObject (|VaRestSubsystem) _returnvalue_2))
      ;[0 0 0] Rim Color
      (LocalVariables|SetObject _returnvalue_3)
      (Variables|Modify|SetRimColor (Utilities|Struct|MakeLinearColor (Utilities|Array|Get(acopy) (Class|VaRestJsonObject|GetNumberArrayField _returnvalue_3 "Rim")) (Utilities|Array|Get(acopy) (Class|VaRestJsonObject|GetNumberArrayField _returnvalue_3 "Rim") 1) (Utilities|Array|Get(acopy) (Class|VaRestJsonObject|GetNumberArrayField _returnvalue_3 "Rim") 2) (Utilities|Array|Get(acopy) (Class|VaRestJsonObject|GetNumberArrayField _returnvalue_3 "Rim") 3)))
      ;[0 0 0] Window Color
      (Variables|Modify|SetScreenColor (Utilities|Struct|MakeLinearColor (Utilities|Array|Get(acopy) (Class|VaRestJsonObject|GetNumberArrayField (LocalVariables|GetObject) "Screen")) (Utilities|Array|Get(acopy) (Class|VaRestJsonObject|GetNumberArrayField (LocalVariables|GetObject) "Screen") 1) (Utilities|Array|Get(acopy) (Class|VaRestJsonObject|GetNumberArrayField (LocalVariables|GetObject) "Screen") 2) (Utilities|Array|Get(acopy) (Class|VaRestJsonObject|GetNumberArrayField (LocalVariables|GetObject) "Screen") 3)))
      ;[0 0 0] Ship Color
      (if (Class|KismetMathLibrary|LinearColorIsNearEqual :A (Utilities|Struct|MakeLinearColor (Utilities|Array|Get(acopy) (Class|VaRestJsonObject|GetNumberArrayField (LocalVariables|GetObject) "Light")) (Utilities|Array|Get(acopy) (Class|VaRestJsonObject|GetNumberArrayField (LocalVariables|GetObject) "Light") 1) (Utilities|Array|Get(acopy) (Class|VaRestJsonObject|GetNumberArrayField (LocalVariables|GetObject) "Light") 2) (Utilities|Array|Get(acopy) (Class|VaRestJsonObject|GetNumberArrayField (LocalVariables|GetObject) "Light") 3)) :Tolerance 0.1)
        (Variables|Modify|SetLightColor "(R=1.000000,G=1.000000,B=1.000000,A=1.000000)")
        (else
          (Variables|Modify|SetLightColor (Utilities|Struct|MakeLinearColor (Utilities|Array|Get(acopy) (Class|VaRestJsonObject|GetNumberArrayField (LocalVariables|GetObject) "Light")) (Utilities|Array|Get(acopy) (Class|VaRestJsonObject|GetNumberArrayField (LocalVariables|GetObject) "Light") 1) (Utilities|Array|Get(acopy) (Class|VaRestJsonObject|GetNumberArrayField (LocalVariables|GetObject) "Light") 2) (Utilities|Array|Get(acopy) (Class|VaRestJsonObject|GetNumberArrayField (LocalVariables|GetObject) "Light") 3))))))
    (:then_1
      (Default|SetColor _backcamera (Variables|Modify|GetScreenColor))
      (Default|SetColor (Variables|/Game/Character/Ship/Screens/BP_BackScreen.BP_BackScreen_C|GetGPS _backcamera) (Variables|Modify|GetScreenColor))
      (Default|SetColor (Variables|/Game/Character/Ship/Screens/BP_BackScreen.BP_BackScreen_C|GetRadar _backcamera) (Variables|Modify|GetScreenColor))
      (Rendering|Components|Light|SetLightColor (Variables|Default|GetPointLight) (Variables|Modify|GetLightColor) true))))

(fn SaveColors
  (bind _array (Modify|ColortoArray (Variables|Modify|GetLightColor)))
  (bind _array_2 (Modify|ColortoArray (Variables|Modify|GetScreenColor)))
  (bind _array_3 (Modify|ColortoArray (Variables|Modify|GetRimColor)))
  (bind _outactors (Actor|GetAllActorsOfClass "/Script/CombatGame.CustomFileHelper"))
  (Class|CustomFileHelper|SaveFile (Utilities|Array|Get(acopy) _outactors) "interior_colors.json" (Class|VaRestJsonObject|EncodeJsontoSingleString (|MakeJson _array _array_2 _array_3)))
  (Development|PrintString (Utilities|String|Append "Saved: " (Class|VaRestJsonObject|EncodeJsontoSingleString (|MakeJson _array _array_2 _array_3)))))

(fn ColortoArray
  (params (Color :type Linear%20Color%20Structure))
  (bind _temparray (LocalVariables|GetTempArray))
  (Utilities|Array|Add _temparray (.r Color))
  (Utilities|Array|Add _temparray (.g Color))
  (Utilities|Array|Add _temparray (.b Color))
  (Utilities|Array|Add _temparray (.a Color))
  (return _temparray))