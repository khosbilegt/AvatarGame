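; Kinect-driven cockpit controls that turn the player's hand movements into ship steering and beam fire, with animated sticks, hands and buttons.
; Each tick, hand X offsets tilt the sticks and drive yaw, while hand heights slide them, their difference driving roll and their sum triggering pitch.
; Hand states pass through a saturating tick counter to debounce each side's firing and grip animation.
; HandleSpeed is an empty stub.
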(event EventTick
  (params (DeltaSeconds :type Float%20%28single-precision%29))
  (Control|HandleShoot)
  (Control|GetHandVectors)
  (Control|HandleYaw)
  (Control|HandleRoll/Pitch)
  (Control|HandleSpeed))

(fn ConstructionScript)

(fn HandleShoot
  (bind _ship (Variables|Default|GetShip))
  (Utilities|FlowControl|Sequence
    (:then_0
      (bind _isvalid (CallFunction|IsValidHold true))
      (if (not _isvalid)
        _
        (else
          (Default|ShootLeftBeam _ship)))
      (Animation|HandleLeftAnimation (not _isvalid)))
    (:then_1
      (bind _isvalid_2 (CallFunction|IsValidHold false))
      (if (not _isvalid_2)
        _
        (else
          (Default|ShootRightBeam _ship)))
      (Animation|HandleRightAnimation (not _isvalid_2)))))

(fn HandleYaw
  (bind _rightvector (Variables|Default|GetRightVector))
  (bind _returnvalue (Math|Float|Clamp(Float) (.x _rightvector) -0.2 0.5))
  (bind _returnvalue_2 (Math|Float|NormalizetoRange _returnvalue -0.2 0.5))
  (bind _returnvalue_3 (- 1.0 _returnvalue_2))
  (bind _returnvalue_4 (* 60 _returnvalue_3))
  (bind _returnvalue_5 (+ _returnvalue_4 -3e+01))
  (Utilities|FlowControl|Sequence
    (:then_0
      ;[0 0 0] Move Sticks
      (bind _output_get (LocalVariables|SetLeftTurn (+ (* 60 (- 1.0 (Math|Float|NormalizetoRange (Math|Float|Clamp(Float) (.x (Variables|Default|GetLeftVector)) -0.5 0.0) -0.5 0.0))) -3e+01)))
      (LocalVariables|SetRightTurn _returnvalue_5)
      (Transformation|SetRelativeRotation (Variables|Default|GetLeftStick) (Math|Rotator|MakeRotator _output_get 0.0 0.0) false false)
      (Transformation|SetRelativeRotation (Variables|Default|GetRightStick) (Math|Rotator|MakeRotator _returnvalue_5 0.0 0.0) false false))
    (:then_1
      ;[0 0 0] Control Ship (Yaw)
      (Pawn|Input|AddControllerYawInput (Variables|Default|GetShip) (/ (+ (LocalVariables|GetLeftTurn) (LocalVariables|GetRightTurn)) -4e+01)))))

(fn HandleRoll/Pitch
  (bind _leftvector (Variables|Default|GetLeftVector))
  (bind _ship (Variables|Default|GetShip))
  (bind _rightvector (Variables|Default|GetRightVector))
  (Utilities|FlowControl|Sequence
    (:then_0
      ;[0 0 0] Move Sticks
      (LocalVariables|SetLeftTurn (.y _leftvector))
      (LocalVariables|SetRightTurn (.y _rightvector))
      (Transformation|SetRelativeLocation (Variables|Default|GetLeftStick) (Math|Vector|MakeVector 0.0 8e+01 (* 50 (.y _leftvector))) false false)
      (Transformation|SetRelativeLocation (Variables|Default|GetRightStick) (Math|Vector|MakeVector 0.0 -8e+01 (* 50 (.y _rightvector))) false false))
    (:then_1
      ;[0 0 0] Control Ship (Roll)
      (Pawn|Input|AddControllerRollInput (Variables|Default|GetShip) (* 2 (+ (LocalVariables|GetLeftTurn) (* -1 (LocalVariables|GetRightTurn))))))
    (:then_2
      ;[0 0 0] Control Ship (Pitch)
      (if (> (+ (LocalVariables|GetLeftTurn) (LocalVariables|GetRightTurn)) 1.8)
        (Pawn|Input|AddControllerPitchInput _ship -1.0)
        (elif (< (+ (LocalVariables|GetLeftTurn) (LocalVariables|GetRightTurn)) 0.2)
          (Pawn|Input|AddControllerPitchInput _ship 1.0))))))

(fn HandleSpeed)

(fn GetHandVectors
  (bind _relativemovement (Default|GetRelativeMovement (Variables|Default|GetKinectCharacter) "NewEnumerator7" "NewEnumerator0"))
  (Variables|Default|SetLeftVector _relativemovement)
  (bind _relativemovement_2 (Default|GetRelativeMovement (Variables|Default|GetKinectCharacter) "NewEnumerator11" "NewEnumerator0"))
  (Variables|Default|SetRightVector _relativemovement_2))

(fn HandleRightAnimation
  (params (isGripped :type Boolean))
  (bind _hand_right (Variables|Default|GetHand_Right))
  (bind _buttonmain_right (Variables|Default|GetButtonMain_Right))
  (bind _returnvalue (Components|SkeletalMesh|GetAnimInstance _hand_right))
  (if isGripped
    (bind _asright_hand_anim_bp (Utilities|Casting|CastToRightHand_AnimBP _returnvalue))
    (Variables|/Game/Models/Mannequin/Animations/RightHand_AnimBP.RightHand_AnimBP_C|SetGripState _asright_hand_anim_bp "NewEnumerator0")
    (Transformation|SetRelativeLocation _buttonmain_right "0,-5.000000, 0" false false)
    (else
      (bind _asright_hand_anim_bp_2 (Utilities|Casting|CastToRightHand_AnimBP _returnvalue))
      (Variables|/Game/Models/Mannequin/Animations/RightHand_AnimBP.RightHand_AnimBP_C|SetGripState _asright_hand_anim_bp_2 "NewEnumerator2")
      (Transformation|SetRelativeLocation _buttonmain_right "0, 0, 0" false false))))

(fn HandleLeftAnimation
  (params (isGripped :type Boolean))
  (bind _hand_left (Variables|Default|GetHand_Left))
  (bind _buttonmain_left (Variables|Default|GetButtonMain_Left))
  (bind _returnvalue (Components|SkeletalMesh|GetAnimInstance _hand_left))
  (if isGripped
    (bind _asright_hand_anim_bp (Utilities|Casting|CastToRightHand_AnimBP _returnvalue))
    (Variables|/Game/Models/Mannequin/Animations/RightHand_AnimBP.RightHand_AnimBP_C|SetGripState _asright_hand_anim_bp "NewEnumerator0")
    (Transformation|SetRelativeLocation _buttonmain_left "0,-5.000000, 0" false false)
    (else
      (bind _asright_hand_anim_bp_2 (Utilities|Casting|CastToRightHand_AnimBP _returnvalue))
      (Variables|/Game/Models/Mannequin/Animations/RightHand_AnimBP.RightHand_AnimBP_C|SetGripState _asright_hand_anim_bp_2 "NewEnumerator2")
      (Transformation|SetRelativeLocation _buttonmain_left "0, 0, 0" false false))))

(fn IsValidHold
  (params (isLeft :type Boolean))
  (bind _kinectcharacter (Variables|Default|GetKinectCharacter))
  (bind _kinecttracker (Variables|/Game/Character/Ship/BP_Pilot.BP_Pilot_C|GetKinectTracker _kinectcharacter))
  (if isLeft
    ;[0 0 0] Left Side
    (bind _returnvalue (Class|KinectActor|GetLeftHandState _kinecttracker))
    (if _returnvalue
      (bind _result (Math|Float|IncrementFloat (Variables|Default|GetLeftReleasedTick))
        (:%20%20
          (bind _output_get (Variables|Default|SetLeftReleasedTick (Math|Float|Clamp(Float) _result -3.0 3.0)))))
      (else
        (bind _result_2 (Math|Float|DecrementFloat (Variables|Default|GetLeftReleasedTick))
          (:%20%20
            (bind _output_get_2 (Variables|Default|SetLeftReleasedTick (Math|Float|Clamp(Float) _result_2 -3.0 3.0)))))))
    (if (== 3.0 _output_get)
      (Variables|Default|SetisLeftNegative false)
      (return (Variables|Default|GetisLeftNegative))
      (elif (== _output_get_2 -3.0)
        (Variables|Default|SetisLeftNegative true)
        (return (Variables|Default|GetisLeftNegative))))
    (else
      ;[0 0 0] Right Side
      (bind _returnvalue_2 (Class|KinectActor|GetRightHandState _kinecttracker))
      (if _returnvalue_2
        (bind _result_3 (Math|Float|IncrementFloat (Variables|Default|GetRightReleasedTick))
          (:%20%20
            (bind _output_get_3 (Variables|Default|SetRightReleasedTick (Math|Float|Clamp(Float) _result_3 -3.0 3.0)))))
        (else
          (bind _result_4 (Math|Float|DecrementFloat (Variables|Default|GetRightReleasedTick))
            (:%20%20
              (bind _output_get_4 (Variables|Default|SetRightReleasedTick (Math|Float|Clamp(Float) _result_4 -3.0 3.0)))))))
      (if (== 3.0 _output_get_3)
        (Variables|Default|SetisRightNegative false)
        (return (Variables|Default|GetisRightNegative))
        (elif (== _output_get_4 -3.0)
          (Variables|Default|SetisRightNegative true)
          (return (Variables|Default|GetisRightNegative)))))))