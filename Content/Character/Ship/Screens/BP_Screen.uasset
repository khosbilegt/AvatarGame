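; BP_Screen is an in-ship screen actor that shows a W_Orientation widget through its widget component.
; On BeginPlay it passes its Ship reference to the widget.
; ChangeHealth writes the clamped health value as text to the widget's HealthBar.
; CustomDestroy tears down the linked Radar and GPS actors along with the screen itself.
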(event Custom|Change%20Health
  (params (Health :type Integer))
  (bind _widget (Variables|Default|GetWidget))
  (bind _returnvalue (UserInterface|GetWidget _widget))
  ;[0 0 0] Sets Health
  (Utilities|IsValid _returnvalue
    (:Is%20Valid
      (bind _asw_orientation (Utilities|Casting|CastToW_Orientation _returnvalue))
      (Rendering|Components|TextRender|SetText (Variables|/Game/Character/Ship/Screens/W_Orientation.W_Orientation_C|GetHealthBar _asw_orientation) (Utilities|Text|ToText(Integer) (Math|Integer|Clamp(Integer) Health 0 100))))))

(event Custom|CustomDestroy
  (Actor|DestroyActor (Variables|Default|GetRadar))
  (Actor|DestroyActor (Variables|Default|GetGPS))
  (Actor|DestroyActor))

(event EventBeginPlay
  ;[0 0 0] Explicitly sets Widget
  (bind _asw_orientation (Utilities|Casting|CastToW_Orientation (UserInterface|GetWidget (Variables|Default|GetWidget))))
  (Variables|/Game/Character/Ship/Screens/W_Orientation.W_Orientation_C|SetShip _asw_orientation (Variables|Default|GetShip)))

(fn ConstructionScript)