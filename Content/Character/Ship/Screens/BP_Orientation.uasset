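; BP_Orientation is a ship screen Blueprint that hosts the W_Orientation widget through its Widget component.
; On BeginPlay it hands its Ship reference to that widget.
; A ChangeHealth event writes the incoming health, clamped to a percentage-style range, into the widget's HealthBar as integer text.
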(event Custom|Change%20Health
  (params (Health :type Integer))
  (bind _widget (Variables|Default|GetWidget))
  (bind _returnvalue (UserInterface|GetWidget _widget))
  (Utilities|IsValid _returnvalue
    (:Is%20Valid
      (bind _asw_orientation (Utilities|Casting|CastToW_Orientation _returnvalue))
      (Rendering|Components|TextRender|SetText (Variables|/Game/Character/Ship/Screens/Widget/W_Orientation.W_Orientation_C|GetHealthBar _asw_orientation) (Utilities|Text|ToText(Integer) (Math|Integer|Clamp(Integer) Health 0 100))))))

(event EventBeginPlay
  (bind _asw_radar (Utilities|Casting|CastToW_Orientation (UserInterface|GetWidget (Variables|Default|GetWidget))))
  (Variables|/Game/Character/Ship/Screens/Widget/W_Orientation.W_Orientation_C|SetShip _asw_radar (Variables|Default|GetShip)))

(fn ConstructionScript)