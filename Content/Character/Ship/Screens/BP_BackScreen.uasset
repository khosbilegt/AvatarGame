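; BP_BackScreen is a ship screen actor that hosts a W_BackCamera widget, presumably for the rear camera view.
; On BeginPlay it passes its Ship reference to that widget.
; SetColor applies a tinted dynamic instance of M_Screen to the Shape component.
; CustomDestroy destroys the associated Radar and GPS actors along with the screen itself.
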(event Custom|Set%20Color
  (params (Color :type Linear%20Color%20Structure))
  (bind _returnvalue (Rendering|Material|CreateDynamicMaterialInstance "/Game/Character/Ship/Screens/Material/M_Screen.M_Screen" "None" "None" :!class /Script/Engine.KismetMaterialLibrary))
  (Rendering|Material|SetVectorParameterValue _returnvalue "Color" Color :!class /Script/Engine.MaterialInstanceDynamic)
  (Rendering|Material|SetMaterial (Variables|Default|GetShape) 0 _returnvalue))

(event Custom|CustomDestroy
  ;[0 0 0] Destroy Function
  (Actor|DestroyActor (Variables|Default|GetRadar))
  (Actor|DestroyActor (Variables|Default|GetGPS))
  (Actor|DestroyActor))

(event EventTick
  (params (DeltaSeconds :type Float%20%28single-precision%29)))

(event EventBeginPlay
  ;[0 0 0] Explicitly sets Widget
  (bind _asw_back_camera (Utilities|Casting|CastToW_BackCamera (UserInterface|GetWidget (Variables|Default|GetWidget))))
  (Variables|/Game/Character/Ship/Screens/Widget/W_BackCamera.W_BackCamera_C|SetShip _asw_back_camera (Variables|Default|GetShip)))

(fn ConstructionScript)