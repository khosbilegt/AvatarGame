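; BP_GPS is a ship screen that tracks the bearing to the level's portal.
; One second after BeginPlay it caches the first BP_Portal and its location, then hands itself to its W_GPS widget.
; Each tick it sets TargetScreenLocation to player control yaw minus look-at yaw from the screen to that cached location.
; The IsModify flag disables both setup and updates.
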(event EventTick
  (params (DeltaSeconds :type Float%20%28single-precision%29))
  (if (not (Variables|Default|GetisModify))
    (Utilities|IsValid (Variables|Default|GetPortal)
      (:Is%20Valid
        (CallFunction|CalculateRotation)))))

(event EventBeginPlay
  (if (not (Variables|Default|GetisModify))
    (Utilities|FlowControl|Delay 1.0)
    (bind _outactors (Actor|GetAllActorsOfClass "/Game/Obstacle/Portal/BP_Portal.BP_Portal_C"))
    (Variables|Default|SetPortal (Utilities|Array|Get(acopy) _outactors))
    (Utilities|IsValid (Utilities|Array|Get(acopy) _outactors)
      (:Is%20Valid
        (Variables|Default|SetTargetLocation (Transformation|GetActorLocation (Utilities|Array|Get(acopy) _outactors)))
        (bind _asw_gps (Utilities|Casting|CastToW_GPS (UserInterface|GetWidget (Variables|Default|GetWidget))))
        (bind _output_get (Variables|Default|SetGPS_Widget _asw_gps))
        (Variables|/Game/Character/Ship/Screens/Widget/W_GPS.W_GPS_C|SetGPS _output_get self)))))

(fn ConstructionScript)

(fn CalculateRotation
  (Variables|Default|SetTargetScreenLocation (- (.yaw (Pawn|GetControlRotation (Game|GetPlayerCharacter 0) :!class /Script/Engine.Pawn)) (.yaw (Math|Rotator|FindLookatRotation (Transformation|GetActorLocation) (Variables|Default|GetTargetLocation))))))