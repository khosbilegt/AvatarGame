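; Kinect tracker Blueprint that exposes body-tracking joint data by named joint.
; GetJointRotator and GetJointVector each switch on a Joint value and return that joint's rotation or position.
; Both map the 25 skeleton joints, from spine base to right thumb, to fixed indices passed into GetJointRotation and GetJointPosition.
; Tick and the construction script are empty, so it serves purely as a lookup layer.
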(event EventTick
  (params (DeltaSeconds :type Float%20%28single-precision%29)))

(fn ConstructionScript)

(fn GetJointRotator
  (params (Joint :type E_JointNameEnum%20Enum :default "NewEnumerator0"))
  (switch Utilities|FlowControl|Switch|SwitchonE_JointNameEnum Joint
    (:NewEnumerator0
      (bind _returnvalue (Class|KinectActor|GetJointRotation))
      (return _returnvalue))
    (:NewEnumerator1
      (bind _returnvalue_2 (Class|KinectActor|GetJointRotation 1))
      (return _returnvalue_2))
    (:NewEnumerator2
      (bind _returnvalue_3 (Class|KinectActor|GetJointRotation 2))
      (return _returnvalue_3))
    (:NewEnumerator3
      (bind _returnvalue_4 (Class|KinectActor|GetJointRotation 3))
      (return _returnvalue_4))
    (:NewEnumerator4
      (bind _returnvalue_5 (Class|KinectActor|GetJointRotation 4))
      (return _returnvalue_5))
    (:NewEnumerator5
      (bind _returnvalue_6 (Class|KinectActor|GetJointRotation 5))
      (return _returnvalue_6))
    (:NewEnumerator6
      (bind _returnvalue_7 (Class|KinectActor|GetJointRotation 6))
      (return _returnvalue_7))
    (:NewEnumerator7
      (bind _returnvalue_8 (Class|KinectActor|GetJointRotation 7))
      (return _returnvalue_8))
    (:NewEnumerator8
      (bind _returnvalue_9 (Class|KinectActor|GetJointRotation 8))
      (return _returnvalue_9))
    (:NewEnumerator9
      (bind _returnvalue_10 (Class|KinectActor|GetJointRotation 9))
      (return _returnvalue_10))
    (:NewEnumerator10
      (bind _returnvalue_11 (Class|KinectActor|GetJointRotation 10))
      (return _returnvalue_11))
    (:NewEnumerator11
      (bind _returnvalue_12 (Class|KinectActor|GetJointRotation 11))
      (return _returnvalue_12))
    (:NewEnumerator12
      (bind _returnvalue_13 (Class|KinectActor|GetJointRotation 12))
      (return _returnvalue_13))
    (:NewEnumerator13
      (bind _returnvalue_14 (Class|KinectActor|GetJointRotation 13))
      (return _returnvalue_14))
    (:NewEnumerator14
      (bind _returnvalue_15 (Class|KinectActor|GetJointRotation 14))
      (return _returnvalue_15))
    (:NewEnumerator15
      (bind _returnvalue_16 (Class|KinectActor|GetJointRotation 15))
      (return _returnvalue_16))
    (:NewEnumerator16
      (bind _returnvalue_17 (Class|KinectActor|GetJointRotation 16))
      (return _returnvalue_17))
    (:NewEnumerator17
      (bind _returnvalue_18 (Class|KinectActor|GetJointRotation 17))
      (return _returnvalue_18))
    (:NewEnumerator18
      (bind _returnvalue_19 (Class|KinectActor|GetJointRotation 18))
      (return _returnvalue_19))
    (:NewEnumerator19
      (bind _returnvalue_20 (Class|KinectActor|GetJointRotation 19))
      (return _returnvalue_20))
    (:NewEnumerator20
      (bind _returnvalue_21 (Class|KinectActor|GetJointRotation 20))
      (return _returnvalue_21))
    (:NewEnumerator21
      (bind _returnvalue_22 (Class|KinectActor|GetJointRotation 21))
      (return _returnvalue_22))
    (:NewEnumerator22
      (bind _returnvalue_23 (Class|KinectActor|GetJointRotation 22))
      (return _returnvalue_23))
    (:NewEnumerator23
      (bind _returnvalue_24 (Class|KinectActor|GetJointRotation 23))
      (return _returnvalue_24))
    (:NewEnumerator24
      (bind _returnvalue_25 (Class|KinectActor|GetJointRotation 24))
      (return _returnvalue_25))))

(fn GetJointVector
  (params (Joint :type E_JointNameEnum%20Enum :default "NewEnumerator0"))
  (switch Utilities|FlowControl|Switch|SwitchonE_JointNameEnum Joint
    (:NewEnumerator0
      (bind _returnvalue (Class|KinectActor|GetJointPosition))
      (return _returnvalue))
    (:NewEnumerator1
      (bind _returnvalue_2 (Class|KinectActor|GetJointPosition 1))
      (return _returnvalue_2))
    (:NewEnumerator2
      (bind _returnvalue_3 (Class|KinectActor|GetJointPosition 2))
      (return _returnvalue_3))
    (:NewEnumerator3
      (bind _returnvalue_4 (Class|KinectActor|GetJointPosition 3))
      (return _returnvalue_4))
    (:NewEnumerator4
      (bind _returnvalue_5 (Class|KinectActor|GetJointPosition 4))
      (return _returnvalue_5))
    (:NewEnumerator5
      (bind _returnvalue_6 (Class|KinectActor|GetJointPosition 5))
      (return _returnvalue_6))
    (:NewEnumerator6
      (bind _returnvalue_7 (Class|KinectActor|GetJointPosition 6))
      (return _returnvalue_7))
    (:NewEnumerator7
      (bind _returnvalue_8 (Class|KinectActor|GetJointPosition 7))
      (return _returnvalue_8))
    (:NewEnumerator8
      (bind _returnvalue_9 (Class|KinectActor|GetJointPosition 8))
      (return _returnvalue_9))
    (:NewEnumerator9
      (bind _returnvalue_10 (Class|KinectActor|GetJointPosition 9))
      (return _returnvalue_10))
    (:NewEnumerator10
      (bind _returnvalue_11 (Class|KinectActor|GetJointPosition 10))
      (return _returnvalue_11))
    (:NewEnumerator11
      (bind _returnvalue_12 (Class|KinectActor|GetJointPosition 11))
      (return _returnvalue_12))
    (:NewEnumerator12
      (bind _returnvalue_13 (Class|KinectActor|GetJointPosition 12))
      (return _returnvalue_13))
    (:NewEnumerator13
      (bind _returnvalue_14 (Class|KinectActor|GetJointPosition 13))
      (return _returnvalue_14))
    (:NewEnumerator14
      (bind _returnvalue_15 (Class|KinectActor|GetJointPosition 14))
      (return _returnvalue_15))
    (:NewEnumerator15
      (bind _returnvalue_16 (Class|KinectActor|GetJointPosition 15))
      (return _returnvalue_16))
    (:NewEnumerator16
      (bind _returnvalue_17 (Class|KinectActor|GetJointPosition 16))
      (return _returnvalue_17))
    (:NewEnumerator17
      (bind _returnvalue_18 (Class|KinectActor|GetJointPosition 17))
      (return _returnvalue_18))
    (:NewEnumerator18
      (bind _returnvalue_19 (Class|KinectActor|GetJointPosition 18))
      (return _returnvalue_19))
    (:NewEnumerator19
      (bind _returnvalue_20 (Class|KinectActor|GetJointPosition 19))
      (return _returnvalue_20))
    (:NewEnumerator20
      (bind _returnvalue_21 (Class|KinectActor|GetJointPosition 20))
      (return _returnvalue_21))
    (:NewEnumerator21
      (bind _returnvalue_22 (Class|KinectActor|GetJointPosition 21))
      (return _returnvalue_22))
    (:NewEnumerator22
      (bind _returnvalue_23 (Class|KinectActor|GetJointPosition 22))
      (return _returnvalue_23))
    (:NewEnumerator23
      (bind _returnvalue_24 (Class|KinectActor|GetJointPosition 23))
      (return _returnvalue_24))
    (:NewEnumerator24
      (bind _returnvalue_25 (Class|KinectActor|GetJointPosition 24))
      (return _returnvalue_25))))