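; Player character that flies a space fighter through Kinect body tracking, with Q and E firing beams from the left and right blasters.
; It spawns a Kinect tracker on BeginPlay and compares joint pairs each tick through GetRelativeMovement.
; Relative joint heights pitch the SpaceFighter up or down within limits at fixed yaw.
; Another joint offset only toggles LeftBeam width, as the movement input code is unconnected.
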(event EventTick
  (params (DeltaSeconds :type Float%20%28single-precision%29))
  (CallFunction|TrackRotation)
  (CallFunction|TrackMovement))

(event EventBeginPlay
  (bind _returnvalue (Game|SpawnActorfromClass "/Game/Kinect/Tracker/BP_KinectTracker.BP_KinectTracker_C" (Transformation|GetActorTransform) "Undefined" 0 0))
  (Variables|Default|SetKinectTracker _returnvalue))

(event Input|KeyboardEvents|Q
  (params (Key :type Key%20Structure :default "None"))
  (bind _leftblaster (Variables|Default|GetLeftBlaster))
  (:Pressed
    (Game|SpawnActorfromClass "/Game/Kinect/Character/BP_Beam.BP_Beam_C" (Math|Transform|MakeTransform (Transformation|GetWorldLocation _leftblaster) (Transformation|GetWorldRotation _leftblaster) "1,1,1") "Undefined" 0 0)))

(event Input|KeyboardEvents|E
  (params (Key :type Key%20Structure :default "None"))
  (bind _rightblaster (Variables|Default|GetRightBlaster))
  (:Pressed
    (Game|SpawnActorfromClass "/Game/Kinect/Character/BP_Beam.BP_Beam_C" (Math|Transform|MakeTransform (Transformation|GetWorldLocation _rightblaster) (Transformation|GetWorldRotation _rightblaster) "1,1,1") "Undefined" 0 0)))

(fn ConstructionScript)

(fn TrackMovement
  (bind _leftbeam (Variables|Default|GetLeftBeam))
  (bind _relativemovement (CallFunction|GetRelativeMovement "NewEnumerator19" "NewEnumerator1"))
  (if (> (.y (* _relativemovement 1e+02)) -9e+01)
    (Niagara|SetNiagaraVariable(Float) _leftbeam "BeamWidth" 5.0)
    (else
      (Niagara|SetNiagaraVariable(Float) _leftbeam "BeamWidth" 1.5))))

(fn TrackRotation
  (bind _spacefighter (Variables|Default|GetSpaceFighter))
  (bind _spacefighter_2 (Variables|Default|GetSpaceFighter))
  (bind _returnvalue (Transformation|GetWorldRotation _spacefighter_2))
  (bind _returnvalue_2 (Transformation|GetWorldRotation _spacefighter))
  (bind _relativemovement (CallFunction|GetRelativeMovement "NewEnumerator11" "NewEnumerator3"))
  (if (> (.z (* _relativemovement 1e+02)) -2e+01)
    (if (>= (.pitch _returnvalue_2) -6e+01)
      (Transformation|SetWorldRotation _spacefighter_2 (Math|Rotator|MakeRotator 0.0 (- (.pitch _returnvalue_2) 2.0) 2.7e+02) false false))
    (else
      (bind _relativemovement_2 (CallFunction|GetRelativeMovement "NewEnumerator7" "NewEnumerator3"))
      (if (> (.z (* _relativemovement_2 1e+02)) -1e+01)
        (if (<= (.pitch _returnvalue) 6e+01)
          (Transformation|SetWorldRotation (Variables|Default|GetSpaceFighter) (Math|Rotator|MakeRotator 0.0 (+ (.pitch _returnvalue) 2.0) 2.7e+02) false false))))))

(fn GetRelativeMovement
  (params (Joint :type E_JointNameEnum%20Enum :default "NewEnumerator0") (RelativeTo :type E_JointNameEnum%20Enum :default "NewEnumerator0"))
  (bind _kinecttracker (Variables|Default|GetKinectTracker))
  (bind _result (Default|GetJointVector _kinecttracker Joint))
  (bind _result_2 (Default|GetJointVector _kinecttracker RelativeTo))
  (return (- _result _result_2)))