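; BP_Wheel is a wheel actor, tied to a Ship, meant to respond to Kinect hand grips.
; Each tick, HandleGrip reads the left hand state from the Ship's KinectTracker and checks whether the Box overlaps the Kinect character's left-hand collision.
; That grip branch is empty, so rotation comes only from the 0 key, which adds a fixed roll step to Root.
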(event EventTick
  (params (DeltaSeconds :type Float%20%28single-precision%29))
  (CallFunction|HandleGrip))

(event Input|KeyboardEvents|0
  (params (Key :type Key%20Structure :default "None"))
  (bind _root (Variables|Default|GetRoot))
  (bind _returnvalue (Transformation|GetRelativeTransform _root))
  (:Pressed
    (Transformation|SetRelativeRotation _root (Math|Rotator|MakeRotator (+ (.roll (.rotation _returnvalue)) 1e+01) (.pitch (.rotation _returnvalue)) (.yaw (.rotation _returnvalue))) false false)))

(fn ConstructionScript)

(fn HandleGrip
  (bind _returnvalue (Class|KinectActor|GetLeftHandState (Variables|/Game/Kinect/Character/BP_Ship.BP_Ship_C|GetKinectTracker (Variables|Default|GetShip))))
  (if (and (Class|PrimitiveComponent|IsOverlappingComponent (Variables|Default|GetBox) (Variables|/Game/Kinect/Character/BP_Character.BP_Character_C|GetLeftCollision (Variables|Default|GetKinectCharacter))) _returnvalue)
    _))