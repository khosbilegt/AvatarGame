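; BP_BlasterBeam is a blaster projectile that damages or knocks BP_Debris actors through their Impact call.
; Each tick it moves its Billboard along the actor's forward vector by Speed, without delta-time scaling.
; On overlapping debris, its Box passes location and direction to Impact, spawns a Niagara explosion and destroys the beam.
; A Delay inside Tick acts as a once-per-second counter that destroys beams after a few seconds.
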(event OnComponentBeginOverlap(Box)
  (params (OverlappedComponent :type Primitive%20Component%20Object%20Reference) (OtherActor :type Actor%20Object%20Reference) (OtherComp :type Primitive%20Component%20Object%20Reference) (OtherBodyIndex :type Integer) (bFromSweep :type Boolean) (SweepResult :type Hit%20Result%20Structure%20%28by%20ref%29))
  (bind _box (Variables|Default|GetBox))
  (bind _returnvalue (Transformation|GetWorldLocation _box))
  (bind _asbp_debris (Utilities|Casting|CastToBP_Debris OtherActor))
  (Default|Impact _asbp_debris _returnvalue (Math|Vector|GetForwardVector _box))
  (Niagara|SpawnSystematLocation "/Game/Models/SpaceFighter/Particle/NS_BlastExplosion.NS_BlastExplosion" _returnvalue)
  (Actor|DestroyActor))

(event EventTick
  (params (DeltaSeconds :type Float%20%28single-precision%29))
  (bind _seconds (Variables|Default|GetSeconds))
  (Transformation|SetWorldLocation (Variables|Default|GetBillboard) (+ (* (Math|Vector|GetForwardVector (Transformation|GetActorRotation)) (Variables|Default|GetSpeed)) (Transformation|GetWorldLocation (Variables|Default|GetBillboard))) false false)
  (Utilities|FlowControl|Delay 1.0)
  (Math|Float|IncrementFloat _seconds
    (:%20%20
      (if (> _seconds 5.0)
        (Actor|DestroyActor)))))

(fn ConstructionScript)