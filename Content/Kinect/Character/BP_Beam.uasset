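; BP_Beam is a short-lived beam actor that travels in a straight line along its facing direction and then removes itself.
; Each Tick offsets the Billboard component along the actor's forward vector by Speed, without sweep or delta-time scaling, so velocity depends on frame rate.
; A one-second Delay inside Tick throttles a Seconds counter, which destroys the actor after roughly six seconds.
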(event EventTick
  (params (DeltaSeconds :type Float%20%28single-precision%29))
  (bind _seconds (Variables|Default|GetSeconds))
  (Transformation|SetWorldLocation (Variables|Default|GetBillboard) (+ (* (Math|Vector|GetForwardVector (Transformation|GetActorRotation)) (Variables|Default|GetSpeed)) (Transformation|GetWorldLocation (Variables|Default|GetBillboard))) false false)
  (Utilities|FlowControl|Delay 1.0)
  (Math|Float|IncrementFloat _seconds
    (:%20%20
      (if (> _seconds 5.0)
        (Actor|DestroyActor)))))

(event EventBeginPlay)

(fn ConstructionScript)