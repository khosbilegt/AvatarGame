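; BP_ImperialShip is an Imperial bot ship obstacle with twin blasters and the Player as its target.
; ShootLeftBeam and ShootRightBeam each spawn a BP_BlasterBeam at their blaster, passing the ship's speed, under independent time-based cooldowns.
; OrientSelf ignores its Target input, sets rotation along the Player-to-ship direction (away from the Player) and prints it.
; ChooseTarget simply returns Player; nothing in this Blueprint calls these events or the function.
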(event Custom|ShootLeftBeam
  (bind _leftblaster (Variables|Default|GetLeftBlaster))
  ;[0 0 0] Blasters
  (if (< (+ (Variables|Default|GetLastLeftBeam) (Math|Timespan|MakeTimespan 0 0 0 0 200)) (Math|DateTime|Now))
    (Variables|Default|SetLastLeftBeam (Math|DateTime|Now))
    (Game|SpawnActorfromClass "/Game/Character/Ship/Ship/BP_BlasterBeam.BP_BlasterBeam_C" (Math|Transform|MakeTransform (Transformation|GetWorldLocation _leftblaster) (Transformation|GetWorldRotation _leftblaster) (Transformation|GetActorScale3D)) "Undefined" 0 (Variables|Default|GetActualSpeed) 0)))

(event Custom|ShootRightBeam
  (bind _returnvalue (Math|DateTime|Now))
  (bind _rightblaster (Variables|Default|GetRightBlaster))
  ;[0 0 0] Blasters
  (if (< (+ (Variables|Default|GetLastRightBeam) (Math|Timespan|MakeTimespan 0 0 0 0 200)) _returnvalue)
    (Variables|Default|SetLastRightBeam _returnvalue)
    (Game|SpawnActorfromClass "/Game/Character/Ship/Ship/BP_BlasterBeam.BP_BlasterBeam_C" (Math|Transform|MakeTransform (Transformation|GetWorldLocation _rightblaster) (Transformation|GetWorldRotation _rightblaster) (Transformation|GetActorScale3D)) "Undefined" 0 (Variables|Default|GetActualSpeed) 0)))

(event Custom|OrientSelf
  (params (Target :type Actor%20Object%20Reference))
  (bind _returnvalue (Transformation|GetActorLocation))
  (bind _player (Variables|Default|GetPlayer))
  (bind _returnvalue_2 (Transformation|GetActorLocation _player))
  (bind _returnvalue_3 (Math|Rotator|FindLookatRotation _returnvalue_2 _returnvalue))
  (Transformation|SetActorRotation _returnvalue_3)
  (Development|PrintString (Utilities|String|ToString(Rotator) _returnvalue_3)))

(fn ConstructionScript)

(fn ChooseTarget
  (return (Variables|Default|GetPlayer)))