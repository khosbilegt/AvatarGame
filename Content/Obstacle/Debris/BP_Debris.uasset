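; BP_Debris is a destructible rock or metal debris obstacle.
; The construction script sets its mesh, and a steel material for metal types, from DebrisType.
; Impact counts hits, swapping to a cracked meteor material, then spawning a Niagara explosion and destroying the actor.
; BeginPlay calls AdjustLocation, which computes an offset near the world axes but never applies it; movement and distance-culling logic is disconnected.
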(event OnComponentBeginOverlap(BigCollision)
  (params (OverlappedComponent :type Primitive%20Component%20Object%20Reference) (OtherActor :type Actor%20Object%20Reference) (OtherComp :type Primitive%20Component%20Object%20Reference) (OtherBodyIndex :type Integer) (bFromSweep :type Boolean) (SweepResult :type Hit%20Result%20Structure%20%28by%20ref%29)))

(event EventBeginPlay
  (CallFunction|AdjustLocation))

(event EventTick
  (params (DeltaSeconds :type Float%20%28single-precision%29)))

(fn ConstructionScript
  (CallFunction|CreateDebris (Variables|Default|GetDebrisType)))

(fn Impact
  (params (Location :type Vector) (Forward :type Vector))
  (bind _output_get (Variables|Default|SetDamage (+ (Variables|Default|GetDamage) 1)))
  (if (== _output_get 2)
    (Rendering|Material|SetMaterial (Variables|Default|GetDebrisMesh) 0 "/Game/Environment/Meteor/M_MeteorCracked.M_MeteorCracked")
    (elif (== (Variables|Default|GetDamage) 5)
      (Niagara|SpawnSystematLocation "/Game/Models/SpaceFighter/Particle/NS_BlastExplosion.NS_BlastExplosion" (Transformation|GetActorLocation) "0, 0, 0" "10.000000,10.000000,10.000000")
      (Actor|DestroyActor))))

(fn CreateDebris
  (params (Type :type E_DebrisTypesEnum%20Enum :default "NewEnumerator0"))
  (bind _debrismesh (Variables|Default|GetDebrisMesh))
  (bind _debrismesh_2 (Variables|Default|GetDebrisMesh))
  (switch Utilities|FlowControl|Switch|SwitchonE_DebrisTypesEnum Type
    (:NewEnumerator0
      (Components|StaticMesh|SetStaticMesh _debrismesh "/Game/SoulCave/Environment/Meshes/Rocks/SM_Cave_Rock_Small01.SM_Cave_Rock_Small01"))
    (:NewEnumerator1
      (Components|StaticMesh|SetStaticMesh _debrismesh "/Game/SoulCave/Environment/Meshes/Rocks/SM_Cave_Rock_Medium01.SM_Cave_Rock_Medium01"))
    (:NewEnumerator2
      (Components|StaticMesh|SetStaticMesh _debrismesh "/Game/SoulCave/Environment/Meshes/Rocks/SM_Cave_Rock_Large02.SM_Cave_Rock_Large02"))
    (:NewEnumerator3
      (Components|StaticMesh|SetStaticMesh _debrismesh_2 "/Game/SoulCave/Environment/Meshes/Rocks/SM_Cave_Rock_Small01.SM_Cave_Rock_Small01")
      (Rendering|Material|SetMaterial _debrismesh_2 0 "/Game/StarterContent/Materials/M_Metal_Steel.M_Metal_Steel"))
    (:NewEnumerator4
      (Components|StaticMesh|SetStaticMesh _debrismesh_2 "/Game/SoulCave/Environment/Meshes/Rocks/SM_Cave_Rock_Large02.SM_Cave_Rock_Large02")
      (Rendering|Material|SetMaterial _debrismesh_2 0 "/Game/StarterContent/Materials/M_Metal_Steel.M_Metal_Steel"))))

(fn AdjustLocation
  (bind _startinggap (Variables|Default|GetStartingGap))
  (bind _startinggap_2 (Variables|Default|GetStartingGap))
  (bind _startinggap_3 (Variables|Default|GetStartingGap))
  (if (Math|Float|InRange(Float) (.x (Transformation|GetActorLocation)) -1e+02 _startinggap)
    (LocalVariables|SetAdjustVector (Math|Vector|MakeVector (+ (.x (LocalVariables|GetAdjustVector)) _startinggap) (.y (LocalVariables|GetAdjustVector)) (.z (LocalVariables|GetAdjustVector)))))
  (if (Math|Float|InRange(Float) (.y (Transformation|GetActorLocation)) -1e+02 _startinggap_3)
    (LocalVariables|SetAdjustVector (Math|Vector|MakeVector (.x (LocalVariables|GetAdjustVector)) (+ (.y (LocalVariables|GetAdjustVector)) _startinggap_3) (.z (LocalVariables|GetAdjustVector)))))
  (if (Math|Float|InRange(Float) (.z (Transformation|GetActorLocation)) -1e+02 _startinggap_2)
    (LocalVariables|SetAdjustVector (Math|Vector|MakeVector (.x (LocalVariables|GetAdjustVector)) (.y (LocalVariables|GetAdjustVector)) (+ (.z (LocalVariables|GetAdjustVector)) _startinggap_2)))))