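; Enemy bot obstacle that flies a randomized looping path while firing twin blasters.
; On BeginPlay it spawns a BP_Spline and, after a short delay, fills it with randomly scattered points scaled from the vector toward the first BP_Portal, closing at its start position.
; Tick advances it along the spline, applies random rotation jitter, wraps at the end, and triggers left and right BP_BlasterBeam spawns throttled by timestamps.
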(event Custom|AddWave
  ;[1 1 1] Prepare Spline
  (for _index (range 1 15)
    (Utilities|Array|Add (Variables|Default|GetSplinePoints) (Utilities|WaveMacro (* (- (Variables|Default|GetTarget) (Variables|Default|GetInitial)) (* _index (/ 1.0 15.0))))))
  (Utilities|Array|Add (Variables|Default|GetSplinePoints) (Variables|Default|GetInitial))
  (Spline|SetSplinePoints (Variables|Default|GetSpline) (Variables|Default|GetSplinePoints) "World" true))

(event Custom|ShootLeftBeam
  (bind _leftblaster (Variables|Default|GetLeftBlaster))
  ;[1 1 1] Blasters
  (if (< (+ (Variables|Default|GetLastLeftBeam) (Math|Timespan|MakeTimespan 0 0 0 0 200)) (Math|DateTime|Now))
    (Variables|Default|SetLastLeftBeam (Math|DateTime|Now))
    (Game|SpawnActorfromClass "/Game/Character/Ship/Ship/BP_BlasterBeam.BP_BlasterBeam_C" (Math|Transform|MakeTransform (Transformation|GetWorldLocation _leftblaster) (Transformation|GetWorldRotation _leftblaster) (Transformation|GetActorScale3D)) "Undefined" 0 (Variables|Default|GetActualSpeed) 1e+01 0)))

(event Custom|ShootRightBeam
  (bind _returnvalue (Math|DateTime|Now))
  (bind _rightblaster (Variables|Default|GetRightBlaster))
  ;[1 1 1] Blasters
  (if (< (+ (Variables|Default|GetLastRightBeam) (Math|Timespan|MakeTimespan 0 0 0 0 200)) _returnvalue)
    (Variables|Default|SetLastRightBeam _returnvalue)
    (Game|SpawnActorfromClass "/Game/Character/Ship/Ship/BP_BlasterBeam.BP_BlasterBeam_C" (Math|Transform|MakeTransform (Transformation|GetWorldLocation _rightblaster) (Transformation|GetWorldRotation _rightblaster) (Transformation|GetActorScale3D)) "Undefined" 0 (Variables|Default|GetActualSpeed) 1e+01 0)))

(event Custom|PrepareSpline
  ;[1 1 1] Prepare Spline
  (Utilities|FlowControl|Delay 2.0)
  (bind _outactors (Actor|GetAllActorsOfClass "/Game/Obstacle/Portal/BP_Portal.BP_Portal_C"))
  (Variables|Default|SetTarget (Transformation|GetActorLocation (Utilities|Array|Get(acopy) _outactors)))
  (bind _output_get (Variables|Default|SetInitial (Transformation|GetActorLocation)))
  (Utilities|Array|Add (Variables|Default|GetSplinePoints) _output_get)
  (CallFunction|AddWave))

(event EventBeginPlay
  (bind _returnvalue (Game|SpawnActorfromClass "/Game/UI/MenuShip/BP_Spline.BP_Spline_C" (Transformation|GetActorTransform) "Undefined" 0 0))
  (Variables|Default|SetSpline (Variables|/Game/UI/MenuShip/BP_Spline.BP_Spline_C|GetSpline _returnvalue))
  (CallFunction|PrepareSpline))

(event EventTick
  (params (DeltaSeconds :type Float%20%28single-precision%29))
  (Variables|Default|SetDistance (+ (* DeltaSeconds (Variables|Default|GetSpeed)) (Variables|Default|GetDistance)))
  (Transformation|SetActorLocation (.location (Spline|GetTransformatDistanceAlongSpline (Variables|Default|GetSpline) (Variables|Default|GetDistance) "World" false)) false false)
  (Class|Actor|AddActorWorldRotation (Utilities|RandomRotator))
  (Utilities|FlowControl|Delay 0.2)
  (CallFunction|ShootLeftBeam)
  (CallFunction|ShootRightBeam)
  (if (> (Variables|Default|GetDistance) (Spline|GetSplineLength (Variables|Default|GetSpline)))
    (Variables|Default|SetDistance 0.0)))

(fn ConstructionScript)