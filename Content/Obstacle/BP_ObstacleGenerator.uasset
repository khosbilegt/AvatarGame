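; Obstacle generator actor that scatters randomly typed debris through the space around the world origin when play begins.
; GenerateDebris spawns BP_Debris at random positions in a large cube with random rotations, passing itself as owner and generator.
; RandomDebrisType truncates a random float to pick the type, so the default fifth type almost never occurs.
; GenerateMeteors would spawn BP_DebrisMeteor actors at the origin, but its call is unconnected.
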(event EventBeginPlay
  (CallFunction|GenerateDebris))

(fn ConstructionScript)

(fn GenerateMeteors
  (bind _self self)
  (for _index (range 0 (Variables|Default|GetMeteorCount))
    (bind _randomtype (CallFunction|RandomDebrisType))
    (Game|SpawnActorfromClass "/Game/Obstacle/Meteor/BP_DebrisMeteor.BP_DebrisMeteor_C" (Math|Transform|MakeTransform "0, 0, 0") "Undefined" _self _self _randomtype 0)))

(fn GenerateDebris
  (bind _self self)
  (for _index (range 0 (Variables|Default|GetDebrisCount))
    (bind _randomtype (CallFunction|RandomDebrisType))
    (Game|SpawnActorfromClass "/Game/Obstacle/Debris/BP_Debris.BP_Debris_C" (Math|Transform|MakeTransform (Math|Vector|MakeVector (Math|Random|RandomFloatinRange -1e+04 1e+04) (Math|Random|RandomFloatinRange -1e+04 1e+04) (Math|Random|RandomFloatinRange -1e+04 1e+04)) (Math|Rotator|MakeRotator (Math|Random|RandomFloatinRange -1.8e+02 1.8e+02) (Math|Random|RandomFloatinRange -1.8e+02 1.8e+02) (Math|Random|RandomFloatinRange -1.8e+02 1.8e+02))) "Undefined" _self _self _randomtype 0)))

(fn RandomDebrisType
  (switch int (Math|Float|Truncate (Math|Random|RandomFloatinRange 0.0 4.0))
    (:Default
      (return "NewEnumerator4"))
    (:0
      (return "NewEnumerator0"))
    (:1
      (return "NewEnumerator1"))
    (:2
      (return "NewEnumerator2"))
    (:3
      (return "NewEnumerator3"))))