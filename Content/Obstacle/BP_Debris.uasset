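; BP_Debris is a meteor-like obstacle that cracks and then explodes under repeated impacts.
; On BeginPlay it takes a random rotation, a fixed enlarged scale and a random Mass value.
; Impact counts hits, swapping to a cracked material, then spawning a Niagara blast and destroying the actor at a higher count.
; Forward drift and player-distance cleanup logic is present but disconnected, and Tick and overlap events are empty.
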(event OnComponentBeginOverlap(SphereCollision)
  (params (OverlappedComponent :type Primitive%20Component%20Object%20Reference) (OtherActor :type Actor%20Object%20Reference) (OtherComp :type Primitive%20Component%20Object%20Reference) (OtherBodyIndex :type Integer) (bFromSweep :type Boolean) (SweepResult :type Hit%20Result%20Structure%20%28by%20ref%29)))

(event EventBeginPlay
  (Transformation|SetActorRotation (Math|Rotator|MakeRotator (Math|Random|RandomFloatinRange 0.0 3.6e+02) (Math|Random|RandomFloatinRange 0.0 3.6e+02) (Math|Random|RandomFloatinRange 0.0 3.6e+02)))
  (Transformation|SetActorScale3D "3.000000,3.000000,3.000000")
  (Variables|Default|SetMass (Math|Random|RandomFloatinRange 1.0 1e+01)))

(event EventTick
  (params (DeltaSeconds :type Float%20%28single-precision%29)))

(fn ConstructionScript)

(fn Impact
  (params (Location :type Vector) (Forward :type Vector))
  (bind _output_get (Variables|Default|SetDamage (+ (Variables|Default|GetDamage) 1)))
  (if (== _output_get 2)
    (Rendering|Material|SetMaterial (Variables|Default|GetStaticMesh) 0 "/Game/Environment/Meteor/M_MeteorCracked.M_MeteorCracked")
    (elif (== (Variables|Default|GetDamage) 5)
      (Niagara|SpawnSystematLocation "/Game/Models/SpaceFighter/Particle/NS_BlastExplosion.NS_BlastExplosion" (Transformation|GetActorLocation) "0, 0, 0" "10.000000,10.000000,10.000000")
      (Actor|DestroyActor))))