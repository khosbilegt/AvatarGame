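; Meteor obstacle that drifts through space and damages the player's ship on contact.
; BeginPlay picks a random, unnormalized Direction with only positive components; Tick spins the debris mesh and offsets the actor by Direction times Speed, unscaled by delta time.
; Overlap with the ship's collision passes CalculateDamage to the player, spawns an explosion and destroys the meteor.
; The player distance check on Tick currently does nothing.
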(event OnComponentBeginOverlap(DebrisMesh)
  (params (OverlappedComponent :type Primitive%20Component%20Object%20Reference) (OtherActor :type Actor%20Object%20Reference) (OtherComp :type Primitive%20Component%20Object%20Reference) (OtherBodyIndex :type Integer) (bFromSweep :type Boolean) (SweepResult :type Hit%20Result%20Structure%20%28by%20ref%29))
  (bind _player (Variables|Default|GetPlayer))
  ;[0 0 0] Collision with Player
  (if (== OtherComp (Variables|/Game/Character/Ship/BP_Ship.BP_Ship_C|GetShipCollision _player))
    (bind _damage (CallFunction|CalculateDamage))
    (Default|OnDebrisHit _player _damage)
    (Effects|SpawnEmitteratLocation "/Game/StarterContent/Particles/P_Explosion.P_Explosion" (Transformation|GetActorLocation) "0, 0, 0" "50.000000,50.000000,50.000000")
    (Actor|DestroyActor)))

(event EventBeginPlay
  ;[0 0 0] Set Movement Direction
  (|CallParentFunction)
  (Variables|Default|SetDirection (Math|Vector|MakeVector (Math|Random|RandomFloatinRange 0.0 1.0) (Math|Random|RandomFloatinRange 0.0 1.0) (Math|Random|RandomFloatinRange 0.0 1.0))))

(event EventTick
  (params (DeltaSeconds :type Float%20%28single-precision%29))
  ;[0 0 0] Meteor Movement
  (|CallParentFunction DeltaSeconds)
  (Transformation|AddLocalRotation (Variables|Default|GetDebrisMesh) "1.000000,1.000000,1.000000" false false)
  (Transformation|AddActorWorldOffset (* (Variables|Default|GetDirection) (Variables|Default|GetSpeed)))
  (if (> (Math|Vector|Distance(Vector) (Transformation|GetActorLocation) (Transformation|GetActorLocation (Variables|Default|GetPlayer))) 1e+04)
    _))

(fn ConstructionScript
  (|CallParentFunction))