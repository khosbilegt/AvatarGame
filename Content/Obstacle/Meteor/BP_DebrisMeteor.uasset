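; BP_DebrisMeteor is a meteor debris obstacle that flies in a straight line along its facing direction.
; Its construction script runs the parent's, then sets DebrisType to a fixed enum value.
; Each Tick runs the parent logic, then MoveMeteor offsets the actor a constant distance along its forward vector, without sweep or delta-time scaling, so speed depends on frame rate.
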(event EventBeginPlay
  (|CallParentFunction))

(event Collision|EventActorBeginOverlap
  (params (OtherActor :type Actor%20Object%20Reference)))

(event EventTick
  (params (DeltaSeconds :type Float%20%28single-precision%29))
  (|CallParentFunction DeltaSeconds)
  (CallFunction|MoveMeteor))

(fn ConstructionScript
  (|CallParentFunction)
  (Variables|Default|SetDebrisType "NewEnumerator1"))

(fn MoveMeteor
  (Transformation|AddActorWorldOffset (* (Math|Vector|GetForwardVector (Transformation|GetActorRotation)) 1e+01)))