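; Meteor obstacle actor that drifts through the level in a random direction with a random, non-uniform size.
; On BeginPlay it randomizes its rotation and per-axis scale, then caches the player pawn as a BP_KinectCharacter.
; Each tick it moves along its forward vector by a fixed, frame-rate-dependent step without sweeping.
; It destroys itself once it is too far from the player.
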(event EventBeginPlay
  (bind _returnvalue (Math|Random|RandomFloatinRange 1.0 1e+01))
  (Transformation|SetActorRotation (Math|Rotator|MakeRotator (Math|Random|RandomFloatinRange 0.0 3.6e+02) (Math|Random|RandomFloatinRange 0.0 3.6e+02) (Math|Random|RandomFloatinRange 0.0 3.6e+02)))
  (Transformation|SetActorScale3D (Math|Vector|MakeVector _returnvalue _returnvalue _returnvalue))
  (bind _asbp_kinect_character (Utilities|Casting|CastToBP_KinectCharacter (Game|Player|GetPlayerPawn 0)))
  (Variables|Default|SetPlayer _asbp_kinect_character))

(event EventTick
  (params (DeltaSeconds :type Float%20%28single-precision%29))
  (Transformation|AddActorWorldOffset (* (Transformation|GetActorForwardVector) 1e+01))
  (if (> (Math|Vector|Distance(Vector) (Transformation|GetActorLocation (Variables|Default|GetPlayer)) (Transformation|GetActorLocation)) 1e+04)
    (Actor|DestroyActor)))

(fn ConstructionScript)