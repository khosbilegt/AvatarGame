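; BP_MenuItem is a menu item actor with a mesh, collision box and text label that highlights when a BP_Pilot overlaps it.
; The construction script applies exposed transforms in world space, sets the label and applies the base color.
; Box overlap events switch between hover and base colors through SetColor, which creates a new M_MenuItem dynamic instance on each call.
; StartMotion is empty, and the Ship.TriggerAction call is unconnected.
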(event OnComponentBeginOverlap(Box)
  (params (OverlappedComponent :type Primitive%20Component%20Object%20Reference) (OtherActor :type Actor%20Object%20Reference) (OtherComp :type Primitive%20Component%20Object%20Reference) (OtherBodyIndex :type Integer) (bFromSweep :type Boolean) (SweepResult :type Hit%20Result%20Structure%20%28by%20ref%29))
  ;[0 0 0] Hover Effects
  (Utilities|Casting|CastToBP_Pilot OtherActor)
  (CallFunction|SetColor (Variables|Default|GetHoverColor)))

(event OnComponentEndOverlap(Box)
  (params (OverlappedComponent :type Primitive%20Component%20Object%20Reference) (OtherActor :type Actor%20Object%20Reference) (OtherComp :type Primitive%20Component%20Object%20Reference) (OtherBodyIndex :type Integer))
  ;[0 0 0] Hover Effects
  (Utilities|Casting|CastToBP_Pilot OtherActor)
  (CallFunction|SetColor (Variables|Default|GetMeshColor)))

(fn ConstructionScript
  (bind _textrender (Variables|Default|GetTextRender))
  (Transformation|SetWorldTransform (Variables|Default|GetStaticMesh) (Variables|Default|GetMeshTransform) false false)
  (Transformation|SetWorldTransform (Variables|Default|GetBox) (Variables|Default|GetCollisionTransform) false false)
  (Transformation|SetWorldTransform _textrender (Variables|Default|GetTextTransform) false false)
  (Rendering|Components|TextRender|SetText _textrender (Variables|Default|GetText))
  (CallFunction|SetColor (Variables|Default|GetMeshColor)))

(fn StartMotion)

(fn SetColor
  (params (Color :type Linear%20Color%20Structure))
  (bind _returnvalue (Rendering|Material|CreateDynamicMaterialInstance "/Game/Menu/Item/M_MenuItem.M_MenuItem" "None" "None" :!class /Script/Engine.KismetMaterialLibrary))
  (Rendering|Material|SetVectorParameterValue _returnvalue "Color" Color :!class /Script/Engine.MaterialInstanceDynamic)
  (Rendering|Material|SetMaterial (Variables|Default|GetStaticMesh) 0 _returnvalue))