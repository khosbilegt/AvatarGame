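; A ship customisation menu button controlled by Kinect-tracked hands.
; While active, it checks each tick whether the assigned hand is within screen bounds, then slides the button while that hand is held.
; Sliding past a threshold picks a direction, and release cycles the color and applies the item's action to ship materials, screens, light or interior/exterior transition.
; Back saves colors to JSON and moves the character before loading MenuLevel.
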(event EventTick
  (params (DeltaSeconds :type Float%20%28single-precision%29))
  ;[0 0 0] Basic Functions
  (if (Variables|Default|GetisActive)
    (Hover|HoverEffects)
    (Hover|HoverMovement)
    (Hover|HoverResult)
    (Camera|CameraBack)))

(event EventBeginPlay
  (Variables|Ship|SetInitialTransform (Transformation|GetActorTransform)))

(fn ConstructionScript
  (bind _meshcolor (Variables|Mesh|GetMeshColor))
  (bind _textrender (Variables|Default|GetTextRender))
  (Transformation|SetRelativeTransform (Variables|Default|GetButtonMesh) (Variables|Mesh|GetMeshTransform) false false)
  (Transformation|SetRelativeTransform (Variables|Default|GetLeftArrowMesh) (Variables|Mesh|GetLeftArrowTransform) false false)
  (Transformation|SetRelativeTransform (Variables|Default|GetRightArrowMesh) (Variables|Mesh|GetRightArrowTransform) false false)
  (Transformation|SetRelativeTransform _textrender (Variables|Text|GetTextTransform) false false)
  (Rendering|Components|TextRender|SetText _textrender (Variables|Text|GetText))
  (Button|SetMeshColors _meshcolor _meshcolor))

(fn StartMotion
  (params (toRight :type Boolean))
  (if toRight
    (Transformation|AddActorWorldOffset (Variables|Blueprints|GetCharacter) "0,2000.000000, 0")
    (Variables|Ship|SetisInterior true)
    (else
      (Transformation|AddActorWorldOffset (Variables|Blueprints|GetCharacter) "0,-2000.000000, 0")
      (Variables|Ship|SetisInterior false))))

(fn SetMeshColors
  (params (Mesh :type Linear%20Color%20Structure) (Outline :type Linear%20Color%20Structure))
  (bind _returnvalue (Rendering|Material|CreateDynamicMaterialInstance "/Game/Menu/MainMenu/M_MenuItem.M_MenuItem" "None" "None" :!class /Script/Engine.KismetMaterialLibrary))
  (Rendering|Material|SetVectorParameterValue _returnvalue "OutlineColor" Outline :!class /Script/Engine.MaterialInstanceDynamic)
  (Rendering|Material|SetVectorParameterValue _returnvalue "Color" Mesh :!class /Script/Engine.MaterialInstanceDynamic)
  (Rendering|Material|SetMaterial (Variables|Default|GetButtonMesh) 0 _returnvalue))

(fn HoverEffects
  (bind _pilot (Variables|Blueprints|GetPilot))
  (bind _meshcolor (Variables|Mesh|GetMeshColor))
  (bind _heightrange (Variables|Hover|GetHeightRange))
  (bind _pilot_2 (Variables|Blueprints|GetPilot))
  (bind _heightrange_2 (Variables|Hover|GetHeightRange))
  (bind _widthrange (Variables|Hover|GetWidthRange))
  (bind _widthrange_2 (Variables|Hover|GetWidthRange))
  (bind _righthand (Variables|/Game/Character/Ship/Controls/BP_Pilot.BP_Pilot_C|GetRightHand _pilot_2))
  (bind _lefthand (Variables|/Game/Character/Ship/Controls/BP_Pilot.BP_Pilot_C|GetLeftHand _pilot))
  (bind _returnvalue (Transformation|GetWorldLocation _righthand))
  (bind _returnvalue_2 (Transformation|GetWorldLocation _lefthand))
  (if (not (Variables|Default|GetisHolding))
    (if (Variables|Hover|GetisLeft)
      (if (Math|Float|InRange(Float) (.y _returnvalue_2) (.x _widthrange_2) (.y _widthrange_2))
        (if (Math|Float|InRange(Float) (.z _returnvalue_2) (.x _heightrange) (.y _heightrange))
          (Button|SetMeshColors (Variables|Mesh|GetMeshColor) (Variables|Mesh|GetHoverColor) :!label _label)
          (Variables|Default|SetisInside true)
          (if (not (Variables|Default|GetplayedHoverSound))
            (Audio|PlaySoundatLocation "/Game/Sound/MP_Hover.MP_Hover" "0, 0, 0" "0, 0, 0" 1.0 1.0 0.0 0 0 0)
            (Variables|Default|SetplayedHoverSound true))
          (else
            (Button|SetMeshColors _meshcolor _meshcolor :!label _label_2)
            (Variables|Default|SetisInside false)
            (Variables|Default|SetplayedHoverSound false)))
        (else
          (goto _label_2)))
      (elif (Math|Float|InRange(Float) (.y _returnvalue) (.x _widthrange) (.y _widthrange))
        (if (Math|Float|InRange(Float) (.z _returnvalue) (.x _heightrange_2) (.y _heightrange_2))
          (goto _label)
          (else
            (goto _label_2)))
        (else
          (goto _label_2))))))

(fn HoverMovement
  (bind _pilot (Variables|Blueprints|GetPilot))
  (bind _meshtransform (Variables|Mesh|GetMeshTransform))
  (bind _arrowhover (Variables|Mesh|GetArrowHover))
  (if (Variables|Default|GetisInside)
    (if (Variables|Hover|GetisLeft)
      (bind _returnvalue (Class|KinectActor|GetLeftHandState (Variables|/Game/Character/Ship/Controls/BP_Pilot.BP_Pilot_C|GetKinectTracker (Variables|Blueprints|GetPilot))))
      (bind _output_get (Variables|Default|SetisHolding _returnvalue))
      (if _output_get
        (Transformation|SetRelativeLocation (Variables|Default|GetButtonMesh) (Utilities|LeftMovement) false false)
        (else
          (Transformation|SetRelativeLocation (Variables|Default|GetButtonMesh) (.location (Variables|Mesh|GetMeshTransform)) false false :!label _label)
          (if (Variables|Default|GetisChosen)
            (CallFunction|ModifyAction)
            (Variables|Default|SetisChosen false))))
      (else
        (bind _returnvalue_2 (Class|KinectActor|GetRightHandState (Variables|/Game/Character/Ship/Controls/BP_Pilot.BP_Pilot_C|GetKinectTracker _pilot)))
        (bind _output_get_2 (Variables|Default|SetisHolding _returnvalue_2))
        (if _output_get_2
          (Transformation|SetRelativeLocation (Variables|Default|GetButtonMesh) (Math|Vector|MakeVector (+ (+ (- (.x (.location (Variables|Mesh|GetMeshTransform))) 4e+01) _arrowhover) (* _arrowhover (Math|Float|NormalizetoRange (.y (Variables|/Script/Engine.SceneComponent|GetRelativeLocation (Variables|/Game/Character/Ship/Controls/BP_Pilot.BP_Pilot_C|GetRightHand _pilot))) 2e+01 3e+01))) (.y (.location _meshtransform)) (.z (.location _meshtransform))) false false)
          (else
            (goto _label)))))
    (else
      (Variables|Default|SetisHolding false))))

(fn HoverResult
  (if (> (.x (Variables|/Script/Engine.SceneComponent|GetRelativeLocation (Variables|Default|GetButtonMesh))) (+ (.x (.location (Variables|Mesh|GetMeshTransform))) (* (Variables|Mesh|GetArrowHover) 0.8)))
    (Variables|Default|SetisPositive true)
    (Variables|Default|SetisChosen true :!label _label)
    (elif (< (.x (Variables|/Script/Engine.SceneComponent|GetRelativeLocation (Variables|Default|GetButtonMesh))) (+ (.x (.location (Variables|Mesh|GetMeshTransform))) (* (Variables|Mesh|GetArrowHover) -0.6)))
      (Variables|Default|SetisPositive false)
      (goto _label))))

(fn ModifyAction
  (Audio|PlaySoundatLocation "/Game/Sound/MP_Select.MP_Select" "0, 0, 0" "0, 0, 0" 1.0 1.0 0.0 0 0 0)
  (Color|ChangeShipColor)
  (Ship|FadeProc)
  (Color|ChangeScreenColor)
  (if (Utilities|Enum|Equal(Enum) (Variables|Blueprints|GetItemAction) "NewEnumerator4")
    (Variables|Ship|SetisBacking true)
    (Color|SaveColorJSON)))

(fn EnumtoColor
  (switch Utilities|FlowControl|Switch|SwitchonE_ColorsEnum (Utilities|Array|Get(acopy) (Variables|Color|GetColorList) (Variables|Color|GetColorIndex))
    (:NewEnumerator0
      (return ""))
    (:NewEnumerator1
      (return "(R=1.000000,G=1.000000,B=1.000000,A=1.000000)"))
    (:NewEnumerator2
      (return "(R=1.000000,G=0.000000,B=0.000000,A=1.000000)"))))

(fn ChangeColor
  (if (Variables|Default|GetisPositive)
    (if (== (Utilities|Array|LastIndex (Variables|Color|GetColorList)) (Variables|Color|GetColorIndex))
      (Variables|Color|SetColorIndex 0)
      (else
        (Variables|Color|SetColorIndex (+ (Variables|Color|GetColorIndex) 1))))
    (elif (== (Variables|Color|GetColorIndex) 0)
      (Variables|Color|SetColorIndex (Utilities|Array|LastIndex (Variables|Color|GetColorList)))
      (else
        (Variables|Color|SetColorIndex (- (Variables|Color|GetColorIndex) 1)))))
  (bind _vector (Ship|EnumtoColor))
  (Variables|Color|SetColorCurrent _vector))

(fn SetMaterial
  (params (Name :type Name) (Material :type Material%20Instance%20Object%20Reference))
  (Rendering|Material|SetMaterialbyName (Variables|/Game/Menu/MenuShip/BP_ShipExterior.BP_ShipExterior_C|GetStaticMesh (Variables|Blueprints|GetShip)) Name Material))

(fn FadeProc
  (bind _ship (Variables|Blueprints|GetShip))
  (switch Utilities|FlowControl|Switch|SwitchonE_ModifyActions (Variables|Blueprints|GetItemAction)
    (:NewEnumerator3
      (Variables|/Game/Menu/MenuShip/BP_ShipExterior.BP_ShipExterior_C|SetdeltaSeconds _ship 0.0)
      (Default|TriggerAction _ship "NewEnumerator4")
      (Variables|Ship|SetisInterior true))
    (:NewEnumerator9
      (Variables|/Game/Menu/MenuShip/BP_ShipExterior.BP_ShipExterior_C|SetdeltaSeconds _ship 0.0)
      (Default|TriggerAction _ship "NewEnumerator5")
      (Variables|Ship|SetisInterior false))))

(fn CameraBack
  (if (Variables|Ship|GetisBacking)
    (if (>= (Variables|Default|GetTotalDistance) 2.5e+02)
      (Default|OpenLevelWrapper (Variables|Blueprints|GetShip) "MenuLevel")
      (else
        (bind _output_get (Variables|Default|SetTotalDistance (+ (Variables|Default|GetTotalDistance) 1e+01)))
        (Transformation|AddActorWorldOffset (Variables|Blueprints|GetCharacter) (Math|Vector|MakeVector _output_get 0.0 0.0))))))

(fn Replace
  (params (Transform :type Transform) (isHidden :type Boolean) (deltaSeconds :type Float%20%28single-precision%29) (replacedWith :type BP%20Modify%20Menu%20Item%20Object%20Reference))
  (Transformation|SetActorLocation (Math|Interpolation|VInterpTo (Transformation|GetActorLocation) (.location Transform) deltaSeconds 0.5) false false)
  (Transformation|SetActorScale3D (Math|Interpolation|VInterpTo (Transformation|GetActorScale3D) (.scale Transform) deltaSeconds 0.5))
  (if (Math|Vector|Equal(Vector) (Transformation|GetActorLocation) (.location Transform) 0.0001)
    (Rendering|SetActorHiddenInGame isHidden)
    (Rendering|SetActorHiddenInGame replacedWith (not isHidden))))

(fn ChangeShipColor
  (bind _ship (Variables|Blueprints|GetShip))
  (bind _colorcurrent (Variables|Color|GetColorCurrent))
  (bind _returnvalue (Rendering|Material|CreateDynamicMaterialInstance "/Game/Menu/MenuShip/M_ShipColor.M_ShipColor" "None" "None" :!class /Script/Engine.KismetMaterialLibrary))
  (bind _output_get (LocalVariables|SetMaterial _returnvalue))
  (Ship|ChangeColor)
  (Rendering|Material|SetVectorParameterValue _output_get "Color" (Variables|Color|GetColorCurrent) :!class /Script/Engine.MaterialInstanceDynamic)
  (switch Utilities|FlowControl|Switch|SwitchonE_ModifyActions (Variables|Blueprints|GetItemAction)
    (:NewEnumerator0
      (Ship|SetMaterial "Metal" (LocalVariables|GetMaterial))
      (Default|SetColor _ship _colorcurrent 1)
      (Variables|Color|SetShipColor _colorcurrent))
    (:NewEnumerator1
      (Ship|SetMaterial "DarkWindow" (LocalVariables|GetMaterial))
      (Default|SetColor _ship _colorcurrent 2)
      (Variables|Color|SetWindowColor _colorcurrent))
    (:NewEnumerator2
      (Ship|SetMaterial "MetalDark" (LocalVariables|GetMaterial))
      (Default|SetColor _ship _colorcurrent 3)
      (Variables|Color|SetWindowColor _colorcurrent))))

(fn ChangeScreenColor
  (bind _colorcurrent (Variables|Color|GetColorCurrent))
  (bind _ship (Variables|Blueprints|GetShip))
  (switch Utilities|FlowControl|Switch|SwitchonE_ModifyActions (Variables|Blueprints|GetItemAction)
    (:NewEnumerator6
      (Default|SetColor (Variables|/Game/Menu/MenuShip/BP_ShipExterior.BP_ShipExterior_C|GetBackScreen _ship) _colorcurrent)
      (Default|SetColor (Variables|/Game/Menu/MenuShip/BP_ShipExterior.BP_ShipExterior_C|GetOrientation _ship) _colorcurrent)
      (Default|SetColor (Variables|/Game/Menu/MenuShip/BP_ShipExterior.BP_ShipExterior_C|GetGPS _ship) _colorcurrent)
      (Variables|Color|SetScreenColor _colorcurrent))
    (:NewEnumerator8
      (Rendering|Components|Light|SetLightColor (Variables|/Script/Engine.Light|GetLightComponent (Variables|/Game/Menu/MenuShip/BP_ShipExterior.BP_ShipExterior_C|GetShipLight (Variables|Blueprints|GetShip))) _colorcurrent true)
      (Variables|Color|SetLightColor _colorcurrent))))

(fn SaveColorJSON
  (bind _array (Color|ColortoArray (Variables|Color|GetRimColor)))
  (bind _array_2 (Color|ColortoArray (Variables|Color|GetWindowColor)))
  (bind _array_3 (Color|ColortoArray (Variables|Color|GetShipColor)))
  (bind _array_4 (Color|ColortoArray (Variables|Color|GetScreenColor)))
  (bind _array_5 (Color|ColortoArray (Variables|Color|GetLightColor)))
  (bind _outactors (Actor|GetAllActorsOfClass "/Script/CombatGame.CustomFileHelper"))
  (Class|CustomFileHelper|SaveFile (Utilities|Array|Get(acopy) _outactors) "colors.json" (Class|VaRestJsonObject|EncodeJsontoSingleString (|MakeJson _array _array_2 _array_3 _array_4 _array_5))))

(fn ColortoArray
  (params (LinearColor :type Linear%20Color%20Structure))
  (bind _temparray (LocalVariables|GetTempArray))
  (Utilities|Array|Add _temparray (.r LinearColor))
  (Utilities|Array|Add _temparray (.g LinearColor))
  (Utilities|Array|Add _temparray (.b LinearColor))
  (Utilities|Array|Add _temparray (.a LinearColor))
  (return _temparray))