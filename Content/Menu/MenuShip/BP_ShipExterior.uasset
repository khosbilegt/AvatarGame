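; Exterior of the menu ship, which animates menu choices and transitions between exterior and interior views.
; TriggerAction sets a Motion state that Tick runs: Start, Modify and Fight follow splines, with Start and Modify also opening levels through a fade widget.
; Fade states crossfade dynamic materials and lights against the linked Ship and swap interior/exterior buttons.
; Rim, window and hull colors load from JSON via VaRest, and SaveColors writes them back.
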(event Custom|Set%20Color
  (params (Color :type Linear%20Color%20Structure) (Elem :type Integer))
  ;[0 0 0] Set Color
  (Utilities|Array|SetArrayElem (Variables|Default|GetColors) Elem Color))

(event Custom|Trigger%20Action
  (params (Motion :type E_MenuActionsEnum%20Enum :default "NewEnumerator0"))
  ;[0 0 0] Sets Motion for Tick
  (Variables|Blueprints|SetMotion Motion)
  (Spline|ChooseSpline)
  (Variables|Default|SetisFaded false)
  (Variables|Default|SetdeltaSeconds 0.0))

(event Custom|Play%20Select
  ;[0 0 0] Select Sound
  (if (not (Variables|Default|GetplayedSound))
    (Audio|PlaySoundatLocation "/Game/Sound/MP_Select.MP_Select" "0, 0, 0" "0, 0, 0" 1.0 1.0 0.0 0 0 0)
    (Variables|Default|SetplayedSound true)))

(event Custom|OpenLevelWrapper
  (params (LevelName :type Name))
  ;[0 0 0] Fade Out Effect
  (bind _returnvalue (UserInterface|CreateWidget "/Game/Menu/EndMenu/W_FadeOut.W_FadeOut_C" 0 LevelName))
  (UserInterface|Viewport|AddtoViewport _returnvalue 0))

(event EventBeginPlay
  (Fade|SaveLightIntensities)
  (Colors|SetColors))

(event EventTick
  (params (DeltaSeconds :type Float%20%28single-precision%29))
  ;[0 0 0] Starts setting delta seconds for motions
  (switch Utilities|FlowControl|Switch|SwitchonE_MenuActionsEnum (Variables|Blueprints|GetMotion)
    (:NewEnumerator1
      (Variables|Default|SetdeltaSeconds (+ DeltaSeconds (Variables|Default|GetdeltaSeconds)))
      (Spline|StartMotion 1e+03)
      (Utilities|FlowControl|Delay 1.0)
      (CallFunction|PlaySelect)
      (CallFunction|OpenLevelWrapper "GameLevel"))
    (:NewEnumerator2
      (Variables|Default|SetdeltaSeconds (+ DeltaSeconds (Variables|Default|GetdeltaSeconds)))
      (Spline|ModifyMotion 1e+03)
      (Utilities|FlowControl|Delay 0.5)
      (CallFunction|PlaySelect)
      (CallFunction|OpenLevelWrapper "ModLevel"))
    (:NewEnumerator3
      (Variables|Default|SetdeltaSeconds (+ DeltaSeconds (Variables|Default|GetdeltaSeconds)))
      (Spline|FightMotion 5e+02))
    (:NewEnumerator4
      (Variables|Default|SetdeltaSeconds (+ DeltaSeconds (Variables|Default|GetdeltaSeconds)))
      (Fade|FadeOut)
      (Fade|SetIsInterior false))
    (:NewEnumerator5
      (Variables|Default|SetdeltaSeconds (+ DeltaSeconds (Variables|Default|GetdeltaSeconds)))
      (Fade|Fadein)
      (Fade|SetIsInterior true))))

(event Input|KeyboardEvents|1
  (params (Key :type Key%20Structure))
  (:Pressed
    (CallFunction|TriggerAction "NewEnumerator4")))

(event Input|KeyboardEvents|2
  (params (Key :type Key%20Structure))
  (:Pressed
    (CallFunction|TriggerAction "NewEnumerator5")))

(fn ConstructionScript)

(fn ModifyMotion
  (params (Speed :type Float%20%28single-precision%29))
  (bind _returnvalue (Transformation|GetActorRotation))
  (Transformation|SetWorldTransform (Variables|Default|GetStaticMesh) (Math|Transform|MakeTransform (.location (Spline|GetTransformatDistanceAlongSpline (Variables|Default|GetUseSpline) (* 0.0 (Math|Interpolation|FInterpTo Speed (* 5 Speed) 0.0 1.0)) "World" false)) (Math|Rotator|MakeRotator (.roll _returnvalue) (.pitch _returnvalue) (Math|Interpolation|FInterpTo (.yaw _returnvalue) 9e+01 0.0 2.0)) (* (Variables|Default|GetShipScale) (+ 0.0 1.0))) false false))

(fn StartMotion
  (params (Speed :type Float%20%28single-precision%29))
  (bind _staticmesh (Variables|Default|GetStaticMesh))
  (bind _returnvalue (Transformation|GetWorldRotation _staticmesh))
  (if (> (.yaw _returnvalue) 159.0)
    (LocalVariables|SetFullSpeed (Math|Interpolation|FInterpTo (LocalVariables|GetFullSpeed) (* 3 (LocalVariables|GetFullSpeed)) 0.0 1.2)))
  (Transformation|SetWorldLocationAndRotation (Variables|Default|GetStaticMesh) (.location (Spline|GetTransformatDistanceAlongSpline (Variables|Default|GetUseSpline) (* 0.0 (* (LocalVariables|GetFullSpeed) Speed)) "World" false)) (Math|Rotator|MakeRotator (.roll _returnvalue) (.pitch _returnvalue) (Math|Interpolation|FInterpTo (.yaw _returnvalue) 1.6e+02 0.0 0.3)) false false)
  (Development|PrintString (Utilities|String|ToString(Float) 0.0)))

(fn FightMotion
  (params (Speed :type Float%20%28single-precision%29))
  (Transformation|SetWorldLocationAndRotation (Variables|Default|GetStaticMesh) (.location (Spline|GetTransformatDistanceAlongSpline (Variables|/Game/Menu/MenuShip/BP_Spline.BP_Spline_C|GetSpline (Variables|Spline|GetFightSpline)) (* 0.0 Speed) "World" false)) (Transformation|GetActorRotation) false false))

(fn ChooseSpline
  (switch Utilities|FlowControl|Switch|SwitchonE_MenuActionsEnum (Variables|Blueprints|GetMotion)
    (:NewEnumerator1
      (Variables|Default|SetUseSpline (Variables|/Game/Menu/MenuShip/BP_Spline.BP_Spline_C|GetSpline (Variables|Spline|GetStartSpline))))
    (:NewEnumerator2
      (Variables|Default|SetUseSpline (Variables|/Game/Menu/MenuShip/BP_Spline.BP_Spline_C|GetSpline (Variables|Spline|GetModifySpline))))))

(fn FadeOut
  (bind _staticmesh (Variables|Default|GetStaticMesh))
  (bind _ship (Variables|Blueprints|GetShip))
  (bind _deltaseconds (Variables|Default|GetdeltaSeconds))
  (bind _returnvalue (/ _deltaseconds 3.0))
  (bind _returnvalue_2 (+ 0.0 _returnvalue))
  (if (not (Variables|Default|GetisFaded))
    (for (_ _array_index) (Rendering|Material|GetMaterials _staticmesh)
      (bind _returnvalue_3 (Rendering|Material|CreateDynamicMaterialInstance _staticmesh 0 "/Game/Menu/MenuShip/M_ShipColor.M_ShipColor" "None" :!class /Script/Engine.PrimitiveComponent))
      (bind _output_get (Variables|Default|SetMaterialInstance _returnvalue_3))
      (Rendering|Material|SetScalarParameterValue _output_get "Appearance" _returnvalue_2 :!class /Script/Engine.MaterialInstanceDynamic)
      (Rendering|Material|SetVectorParameterValue (Variables|Default|GetMaterialInstance) "Color" (Utilities|Array|Get(acopy) (Variables|Default|GetColors) _array_index) :!class /Script/Engine.MaterialInstanceDynamic)
      (Rendering|Material|SetMaterial (Variables|Default|GetStaticMesh) _array_index (Variables|Default|GetMaterialInstance))
      (Fade|SetLightIntensities _returnvalue_2)
      (if (> _returnvalue_2 1.0)
        (Variables|Default|SetisFaded true)
        (else
          (Utilities|IsValid _ship
            (:Is%20Valid
              (Default|Fadein _ship (Variables|Default|GetdeltaSeconds)))))))))

(fn Fadein
  (bind _staticmesh (Variables|Default|GetStaticMesh))
  (bind _ship (Variables|Blueprints|GetShip))
  (bind _deltaseconds (Variables|Default|GetdeltaSeconds))
  (bind _returnvalue (/ _deltaseconds 3.0))
  (bind _returnvalue_2 (- 1.0 _returnvalue))
  (if (not (Variables|Default|GetisFaded))
    (for (_ _array_index) (Rendering|Material|GetMaterials _staticmesh)
      (bind _returnvalue_3 (Rendering|Material|CreateDynamicMaterialInstance _staticmesh 0 "/Game/Menu/MenuShip/M_ShipColor.M_ShipColor" "None" :!class /Script/Engine.PrimitiveComponent))
      (bind _output_get (Variables|Default|SetMaterialInstance _returnvalue_3))
      (Rendering|Material|SetScalarParameterValue _output_get "Appearance" _returnvalue_2 :!class /Script/Engine.MaterialInstanceDynamic)
      (Rendering|Material|SetVectorParameterValue (Variables|Default|GetMaterialInstance) "Color" (Utilities|Array|Get(acopy) (Variables|Default|GetColors) _array_index) :!class /Script/Engine.MaterialInstanceDynamic)
      (Rendering|Material|SetMaterial (Variables|Default|GetStaticMesh) _array_index (Variables|Default|GetMaterialInstance))
      (Fade|SetLightIntensities _returnvalue_2)
      (if (< _returnvalue_2 0.0)
        (Variables|Default|SetisFaded true)
        (else
          (Utilities|IsValid _ship
            (:Is%20Valid
              (Default|FadeOut _ship (Variables|Default|GetdeltaSeconds)))))))))

(fn SaveLightIntensities
  (bind _lights (Variables|Light|GetLights))
  (bind _shiplight (Variables|Light|GetShipLight))
  (bind _lightcomponent (Variables|/Script/Engine.Light|GetLightComponent _shiplight))
  (if (!= (Utilities|Array|Length _lights) 0)
    (for _array_element _lights
      (Utilities|Array|Add (Variables|Light|GetLightIntensities) (Variables|/Script/Engine.LightComponentBase|GetIntensity (Variables|/Script/Engine.Light|GetLightComponent _array_element))))
    (Variables|Default|SetIntensity (Variables|/Script/Engine.LightComponentBase|GetIntensity _lightcomponent))
    (Rendering|Components|Light|SetIntensity _lightcomponent 0.0)))

(fn SetLightIntensities
  (params (Percentage :type Float%20%28single-precision%29))
  (bind _shiplight (Variables|Light|GetShipLight))
  (bind _lightcomponent (Variables|/Script/Engine.Light|GetLightComponent _shiplight))
  (for (_array_element _array_index) (Variables|Light|GetLights)
    (Rendering|Components|Light|SetIntensity (Variables|/Script/Engine.Light|GetLightComponent _array_element) (* (Utilities|Array|Get(acopy) (Variables|Light|GetLightIntensities) _array_index) (- 1.0 Percentage))))
  (Rendering|Components|Light|SetIntensity _lightcomponent (* Percentage (Variables|Default|GetIntensity)))
  (Rendering|Components|Light|SetLightColor _lightcomponent (Variables|/Game/Character/Ship/Ship/BP_Ship.BP_Ship_C|GetLightColor (Variables|Blueprints|GetShip)) true))

(fn SetIsInterior
  (params (isExterior :type Boolean))
  (if isExterior
    (for (_array_element _array_index) (Variables|Buttons|GetInteriorButtons)
      (Rendering|SetActorHiddenInGame _array_element true)
      (Rendering|SetActorHiddenInGame (Utilities|Array|Get(acopy) (Variables|Buttons|GetExteriorButtons) _array_index) false)
      (Default|Replace (Utilities|Array|Get(acopy) (Variables|Buttons|GetExteriorButtons) _array_index) (Variables|/Game/Menu/ModifyMenu/BP_ModifyMenu_Item.BP_ModifyMenu_Item_C|GetInitialTransform (Utilities|Array|Get(acopy) (Variables|Buttons|GetExteriorButtons) _array_index)) true (Variables|Default|GetdeltaSeconds) (Utilities|Array|Get(acopy) (Variables|Buttons|GetExteriorButtons) _array_index))
      (Variables|/Game/Menu/ModifyMenu/BP_ModifyMenu_Item.BP_ModifyMenu_Item_C|SetisActive _array_element false)
      (Variables|/Game/Menu/ModifyMenu/BP_ModifyMenu_Item.BP_ModifyMenu_Item_C|SetisActive (Utilities|Array|Get(acopy) (Variables|Buttons|GetExteriorButtons) _array_index) true))
    (else
      (for (_array_element_2 _array_index_2) (Variables|Buttons|GetExteriorButtons)
        (Default|Replace _array_element_2 (Transformation|GetActorTransform (Utilities|Array|Get(acopy) (Variables|Buttons|GetInteriorButtons) _array_index_2)) true (Variables|Default|GetdeltaSeconds) (Utilities|Array|Get(acopy) (Variables|Buttons|GetInteriorButtons) _array_index_2))
        (Variables|/Game/Menu/ModifyMenu/BP_ModifyMenu_Item.BP_ModifyMenu_Item_C|SetisActive _array_element_2 false)
        (Variables|/Game/Menu/ModifyMenu/BP_ModifyMenu_Item.BP_ModifyMenu_Item_C|SetisActive (Utilities|Array|Get(acopy) (Variables|Buttons|GetInteriorButtons) _array_index_2) true)
        ;[0 0 0] Hide Screens
        (Rendering|SetActorHiddenInGame (Variables|Blueprints|GetBackScreen) isExterior)
        (Rendering|SetActorHiddenInGame (Variables|Blueprints|GetGPS) isExterior)
        (Rendering|SetActorHiddenInGame (Variables|Blueprints|GetOrientation) isExterior)))))

(fn SetColors
  (Utilities|FlowControl|Sequence
    (:then_0
      ;[0 0 0] Handles JSON
      (bind _returnvalue (Game|SpawnActorfromClass "/Script/CombatGame.CustomFileHelper" (Transformation|GetActorTransform) "Undefined" 0 0))
      (bind _returnvalue_2 (Class|CustomFileHelper|LoadFile _returnvalue "external_colors.json"))
      (bind _returnvalue_3 (Class|VaRestSubsystem|DecodeJsonObject (|VaRestSubsystem) _returnvalue_2))
      ;[0 0 0] Rim Color
      (LocalVariables|SetObject _returnvalue_3)
      (Variables|Buttons|SetRimColor_0 (Utilities|Struct|MakeLinearColor (Utilities|Array|Get(acopy) (Class|VaRestJsonObject|GetNumberArrayField _returnvalue_3 "Rim")) (Utilities|Array|Get(acopy) (Class|VaRestJsonObject|GetNumberArrayField _returnvalue_3 "Rim") 1) (Utilities|Array|Get(acopy) (Class|VaRestJsonObject|GetNumberArrayField _returnvalue_3 "Rim") 2) (Utilities|Array|Get(acopy) (Class|VaRestJsonObject|GetNumberArrayField _returnvalue_3 "Rim") 3)))
      ;[0 0 0] Window Color
      (Variables|Colors|SetWindowColor (Utilities|Struct|MakeLinearColor (Utilities|Array|Get(acopy) (Class|VaRestJsonObject|GetNumberArrayField (LocalVariables|GetObject) "Window")) (Utilities|Array|Get(acopy) (Class|VaRestJsonObject|GetNumberArrayField (LocalVariables|GetObject) "Window") 1) (Utilities|Array|Get(acopy) (Class|VaRestJsonObject|GetNumberArrayField (LocalVariables|GetObject) "Window") 2) (Utilities|Array|Get(acopy) (Class|VaRestJsonObject|GetNumberArrayField (LocalVariables|GetObject) "Window") 3)))
      ;[0 0 0] Ship Color
      (Variables|Colors|SetShipColor (Utilities|Struct|MakeLinearColor (Utilities|Array|Get(acopy) (Class|VaRestJsonObject|GetNumberArrayField (LocalVariables|GetObject) "Ship")) (Utilities|Array|Get(acopy) (Class|VaRestJsonObject|GetNumberArrayField (LocalVariables|GetObject) "Ship") 1) (Utilities|Array|Get(acopy) (Class|VaRestJsonObject|GetNumberArrayField (LocalVariables|GetObject) "Ship") 2) (Utilities|Array|Get(acopy) (Class|VaRestJsonObject|GetNumberArrayField (LocalVariables|GetObject) "Ship") 3))))
    (:then_1
      (Colors|SetMeshColor (Variables|Colors|GetWindowColor) "DarkWindow")
      (Colors|SetMeshColor (Variables|Colors|GetShipColor) "Metal")
      (Colors|SetMeshColor (Variables|Buttons|GetRimColor_0) "MetalDark"))))

(fn SetMaterial)

(fn SetMeshColor
  (params (Color :type Linear%20Color%20Structure) (Slot :type Name))
  (bind _returnvalue (Rendering|Material|CreateDynamicMaterialInstance "/Game/Menu/MenuShip/M_ShipColor.M_ShipColor" "None" "None" :!class /Script/Engine.KismetMaterialLibrary))
  (Rendering|Material|SetVectorParameterValue _returnvalue "Color" Color :!class /Script/Engine.MaterialInstanceDynamic)
  (Rendering|Material|SetMaterialbyName (Variables|Default|GetStaticMesh) Slot _returnvalue))

(fn SaveColors
  (bind _array (Colors|ColortoArray (Variables|Buttons|GetRimColor_0)))
  (bind _array_2 (Colors|ColortoArray (Variables|Colors|GetWindowColor)))
  (bind _array_3 (Colors|ColortoArray (Variables|Colors|GetShipColor)))
  (bind _outactors (Actor|GetAllActorsOfClass "/Script/CombatGame.CustomFileHelper"))
  (Class|CustomFileHelper|SaveFile (Utilities|Array|Get(acopy) _outactors) "external_colors.json" (Class|VaRestJsonObject|EncodeJsontoSingleString (|MakeJson _array _array_2 _array_3)))
  (Development|PrintString (Utilities|String|Append "Saved: " (Class|VaRestJsonObject|EncodeJsontoSingleString (|MakeJson _array _array_2 _array_3)))))

(fn ColortoArray
  (params (Color :type Linear%20Color%20Structure))
  (bind _temparray (LocalVariables|GetTempArray))
  (Utilities|Array|Add _temparray (.r Color))
  (Utilities|Array|Add _temparray (.g Color))
  (Utilities|Array|Add _temparray (.b Color))
  (Utilities|Array|Add _temparray (.a Color))
  (return _temparray))