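; Menu ship actor that flies along splines when TriggerAction sets a Start, Modify or Fight motion.
; Tick accumulates time as spline distance: Start eases yaw and speeds up, Modify turns and scales the ship, Fight just follows its own spline.
; Start and Modify open GameLevel and ModLevel after short delays.
; Every tick also rebuilds dynamic M_ShipColor materials, driving Appearance from the accumulated time.
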(event Custom|Trigger%20Action
  (params (Motion :type E_MenuActionsEnum%20Enum :default "NewEnumerator0"))
  ;[0 0 0] Sets Motion for Tick
  (Variables|Default|SetMotion Motion)
  (CallFunction|ChooseSpline))

(event EventBeginPlay)

(event EventTick
  (params (DeltaSeconds :type Float%20%28single-precision%29))
  ;[0 0 0] Starts setting delta seconds for motions
  (Variables|Default|SetDelta%20Seconds (+ DeltaSeconds (Variables|Default|GetDelta%20Seconds)))
  (CallFunction|ColorFunc)
  (switch Utilities|FlowControl|Switch|SwitchonE_MenuActionsEnum (Variables|Default|GetMotion)
    (:NewEnumerator1
      (Variables|Default|SetDelta%20Seconds (+ DeltaSeconds (Variables|Default|GetDelta%20Seconds)))
      (CallFunction|StartMotion 1e+03)
      (Utilities|FlowControl|Delay 1.0)
      (Game|OpenLevel(byName) "GameLevel"))
    (:NewEnumerator2
      (Variables|Default|SetDelta%20Seconds (+ DeltaSeconds (Variables|Default|GetDelta%20Seconds)))
      (CallFunction|ModifyMotion 1e+03)
      (Utilities|FlowControl|Delay 0.5)
      (Game|OpenLevel(byName) "ModLevel"))
    (:NewEnumerator3
      (Variables|Default|SetDelta%20Seconds (+ DeltaSeconds (Variables|Default|GetDelta%20Seconds)))
      (CallFunction|FightMotion 5e+02))))

(fn ConstructionScript)

(fn ModifyMotion
  (params (Speed :type Float%20%28single-precision%29))
  (bind _returnvalue (Transformation|GetActorRotation))
  (bind _delta_seconds (Variables|Default|GetDelta%20Seconds))
  (Transformation|SetWorldTransform (Variables|Default|GetStaticMesh) (Math|Transform|MakeTransform (.location (Spline|GetTransformatDistanceAlongSpline (Variables|Default|GetUseSpline) (* _delta_seconds (Math|Interpolation|FInterpTo Speed (* 5 Speed) _delta_seconds 1.0)) "World" false)) (Math|Rotator|MakeRotator (.roll _returnvalue) (.pitch _returnvalue) (Math|Interpolation|FInterpTo (.yaw _returnvalue) 9e+01 _delta_seconds 2.0)) (* (Variables|Default|GetShipScale) (+ (Variables|Default|GetDelta%20Seconds) 1.0))) false false))

(fn StartMotion
  (params (Speed :type Float%20%28single-precision%29))
  (bind _delta_seconds (Variables|Default|GetDelta%20Seconds))
  (bind _staticmesh (Variables|Default|GetStaticMesh))
  (bind _returnvalue (Transformation|GetWorldRotation _staticmesh))
  (if (> (.yaw _returnvalue) 159.0)
    (LocalVariables|SetFullSpeed (Math|Interpolation|FInterpTo (LocalVariables|GetFullSpeed) (* 3 (LocalVariables|GetFullSpeed)) (Variables|Default|GetDelta%20Seconds) 1.2)))
  (Transformation|SetWorldLocationAndRotation (Variables|Default|GetStaticMesh) (.location (Spline|GetTransformatDistanceAlongSpline (Variables|Default|GetUseSpline) (* _delta_seconds (* (LocalVariables|GetFullSpeed) Speed)) "World" false)) (Math|Rotator|MakeRotator (.roll _returnvalue) (.pitch _returnvalue) (Math|Interpolation|FInterpTo (.yaw _returnvalue) 1.6e+02 _delta_seconds 0.3)) false false)
  (Development|PrintString (Utilities|String|ToString(Float) _delta_seconds)))

(fn FightMotion
  (params (Speed :type Float%20%28single-precision%29))
  (Transformation|SetWorldLocationAndRotation (Variables|Default|GetStaticMesh) (.location (Spline|GetTransformatDistanceAlongSpline (Variables|/Game/Menu/MenuShip/BP_Spline.BP_Spline_C|GetSpline (Variables|Default|GetFightSpline)) (* (Variables|Default|GetDelta%20Seconds) Speed) "World" false)) (Transformation|GetActorRotation) false false))

(fn ChooseSpline
  (switch Utilities|FlowControl|Switch|SwitchonE_MenuActionsEnum (Variables|Default|GetMotion)
    (:NewEnumerator1
      (Variables|Default|SetUseSpline (Variables|/Game/Menu/MenuShip/BP_Spline.BP_Spline_C|GetSpline (Variables|Default|GetStartSpline))))
    (:NewEnumerator2
      (Variables|Default|SetUseSpline (Variables|/Game/Menu/MenuShip/BP_Spline.BP_Spline_C|GetSpline (Variables|Default|GetModifySpline))))))

(fn ColorFunc
  (bind _staticmesh (Variables|Default|GetStaticMesh))
  (for (_ _array_index) (Rendering|Material|GetMaterials _staticmesh)
    (bind _returnvalue (Rendering|Material|CreateDynamicMaterialInstance _staticmesh 0 "/Game/Menu/MenuShip/M_ShipColor.M_ShipColor" "None" :!class /Script/Engine.PrimitiveComponent))
    (bind _output_get (Variables|Default|SetMaterialInstance _returnvalue))
    (Rendering|Material|SetScalarParameterValue _output_get "Appearance" (+ 0.0 (/ (Variables|Default|GetDelta%20Seconds) 3.0)) :!class /Script/Engine.MaterialInstanceDynamic)
    (Rendering|Material|SetMaterial (Variables|Default|GetStaticMesh) _array_index (Variables|Default|GetMaterialInstance))))