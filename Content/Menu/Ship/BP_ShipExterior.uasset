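; BP_ShipExterior is the menu's exterior ship actor, which flies its static mesh along splines for Start, Modify and Fight motions.
; TriggerAction sets the motion state, and Tick accumulates time and calls the matching motion function.
; Each function converts time times speed into distance along its own spline, moving the mesh there while keeping the actor's rotation.
; The accumulated time is shared by all motions and never reset here.
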(event Custom|Trigger%20Action
  (params (Motion :type E_MenuActionsEnum%20Enum :default "NewEnumerator0"))
  ;[0 0 0] Sets Motion for Tick
  (Variables|Default|SetMotion Motion))

(event EventTick
  (params (DeltaSeconds :type Float%20%28single-precision%29))
  ;[0 0 0] Starts setting delta seconds for motions
  (switch Utilities|FlowControl|Switch|SwitchonE_MenuActionsEnum (Variables|Default|GetMotion)
    (:NewEnumerator1
      (Variables|Default|SetDelta%20Seconds (+ DeltaSeconds (Variables|Default|GetDelta%20Seconds)))
      (CallFunction|StartMotion 5e+02))
    (:NewEnumerator2
      (Variables|Default|SetDelta%20Seconds (+ DeltaSeconds (Variables|Default|GetDelta%20Seconds)))
      (CallFunction|ModifyMotion 2e+02))
    (:NewEnumerator3
      (Variables|Default|SetDelta%20Seconds (+ DeltaSeconds (Variables|Default|GetDelta%20Seconds)))
      (CallFunction|FightMotion 5e+02))))

(fn ConstructionScript)

(fn StartMotion
  (params (Speed :type Float%20%28single-precision%29))
  (Transformation|SetWorldLocationAndRotation (Variables|Default|GetStaticMesh) (.location (Spline|GetTransformatDistanceAlongSpline (Variables|/Game/Menu/Ship/BP_Spline.BP_Spline_C|GetSpline (Variables|Default|GetStartSpline)) (* (Variables|Default|GetDelta%20Seconds) Speed) "World" false)) (Transformation|GetActorRotation) false false))

(fn ModifyMotion
  (params (Speed :type Float%20%28single-precision%29))
  (Transformation|SetWorldLocationAndRotation (Variables|Default|GetStaticMesh) (.location (Spline|GetTransformatDistanceAlongSpline (Variables|/Game/Menu/Ship/BP_Spline.BP_Spline_C|GetSpline (Variables|Default|GetModifySpline)) (* (Variables|Default|GetDelta%20Seconds) Speed) "World" false)) (Transformation|GetActorRotation) false false))

(fn FightMotion
  (params (Speed :type Float%20%28single-precision%29))
  (Transformation|SetWorldLocationAndRotation (Variables|Default|GetStaticMesh) (.location (Spline|GetTransformatDistanceAlongSpline (Variables|/Game/Menu/Ship/BP_Spline.BP_Spline_C|GetSpline (Variables|Default|GetFightSpline)) (* (Variables|Default|GetDelta%20Seconds) Speed) "World" false)) (Transformation|GetActorRotation) false false))