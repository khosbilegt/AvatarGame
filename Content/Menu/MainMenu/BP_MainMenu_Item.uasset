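; Main menu button operated by the pilot's Kinect-tracked left hand, triggering an action on the Ship.
; Construction places the button, arrow and text and applies the colors through a dynamic material.
; Each tick, a world Y/Z range check drives the hover outline, arrow nudge and one-shot sound.
; For left-side items, a held hand slides the button along X, and passing 80% of its travel fires the action.
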(event EventTick
  (params (DeltaSeconds :type Float%20%28single-precision%29))
  (CallFunction|HoverEffects)
  (CallFunction|HoverMovement)
  (CallFunction|HoverResult))

(fn ConstructionScript
  (bind _meshcolor (Variables|Mesh|GetMeshColor))
  (bind _textrender (Variables|Default|GetTextRender))
  (Transformation|SetRelativeTransform (Variables|Default|GetButtonMesh) (Variables|Mesh|GetMeshTransform) false false)
  (Transformation|SetRelativeTransform (Variables|Default|GetArrowMesh) (Variables|Mesh|GetArrowTransform) false false)
  (Transformation|SetRelativeTransform _textrender (Variables|Text|GetTextTransform) false false)
  (Rendering|Components|TextRender|SetText _textrender (Variables|Text|GetText))
  (CallFunction|SetColors _meshcolor _meshcolor))

(fn StartMotion)

(fn SetColors
  (params (Mesh :type Linear%20Color%20Structure) (Outline :type Linear%20Color%20Structure))
  (bind _returnvalue (Rendering|Material|CreateDynamicMaterialInstance "/Game/Menu/MainMenu/M_MenuItem.M_MenuItem" "None" "None" :!class /Script/Engine.KismetMaterialLibrary))
  (Rendering|Material|SetVectorParameterValue _returnvalue "OutlineColor" Outline :!class /Script/Engine.MaterialInstanceDynamic)
  (Rendering|Material|SetVectorParameterValue _returnvalue "Color" Mesh :!class /Script/Engine.MaterialInstanceDynamic)
  (Rendering|Material|SetMaterial (Variables|Default|GetButtonMesh) 0 _returnvalue))

(fn HoverEffects
  (bind _arrowmesh (Variables|Default|GetArrowMesh))
  (bind _arrowtransform (Variables|Mesh|GetArrowTransform))
  (bind _meshcolor (Variables|Mesh|GetMeshColor))
  (bind _pilot (Variables|Blueprints|GetPilot))
  (bind _heightrange (Variables|Hover|GetHeightRange))
  (bind _widthrange (Variables|Hover|GetWidthRange))
  (bind _lefthand (Variables|/Game/Character/Ship/Controls/BP_Pilot.BP_Pilot_C|GetLeftHand _pilot))
  (bind _returnvalue (Transformation|GetWorldLocation _lefthand))
  (if (not (Variables|Default|GetisHolding))
    (if (Math|Float|InRange(Float) (.y _returnvalue) (.x _widthrange) (.y _widthrange))
      (if (Math|Float|InRange(Float) (.z _returnvalue) (.x _heightrange) (.y _heightrange))
        (CallFunction|SetColors (Variables|Mesh|GetMeshColor) (Variables|Mesh|GetHoverColor))
        (Transformation|SetRelativeLocation _arrowmesh (Math|Vector|MakeVector (+ (Variables|Mesh|GetArrowHover) (.x (.location _arrowtransform))) (.y (.location _arrowtransform)) (.z (.location _arrowtransform))) false false)
        (Variables|Default|SetisInside true)
        (if (not (Variables|Default|GetplayedSound))
          (Audio|PlaySoundatLocation "/Game/Sound/MP_Hover.MP_Hover" "0, 0, 0" "0, 0, 0" 1.0 1.0 0.0 0 0 0)
          (Variables|Default|SetplayedSound true))
        (else
          (CallFunction|SetColors _meshcolor _meshcolor :!label _label)
          (Transformation|SetRelativeLocation _arrowmesh (.location (Variables|Mesh|GetArrowTransform)) false false)
          (Variables|Default|SetisInside false)
          (Variables|Default|SetplayedSound false)))
      (else
        (goto _label)))))

(fn HoverMovement
  (bind _pilot (Variables|Blueprints|GetPilot))
  (bind _meshtransform (Variables|Mesh|GetMeshTransform))
  (if (Variables|Default|GetisInside)
    (if (Variables|Hover|GetisLeft)
      (bind _returnvalue (Class|KinectActor|GetLeftHandState (Variables|/Game/Character/Ship/Controls/BP_Pilot.BP_Pilot_C|GetKinectTracker _pilot)))
      (bind _output_get (Variables|Default|SetisHolding _returnvalue))
      (if _output_get
        (Transformation|SetRelativeLocation (Variables|Default|GetButtonMesh) (Math|Vector|MakeVector (+ (.x (.location (Variables|Mesh|GetMeshTransform))) (* (Variables|Mesh|GetArrowHover) (Math|Float|NormalizetoRange (.y (Variables|/Script/Engine.SceneComponent|GetRelativeLocation (Variables|/Game/Character/Ship/Controls/BP_Pilot.BP_Pilot_C|GetLeftHand _pilot))) -3e+01 -15.0))) (.y (.location _meshtransform)) (.z (.location _meshtransform))) false false)
        (else
          (Transformation|SetRelativeLocation (Variables|Default|GetButtonMesh) (.location (Variables|Mesh|GetMeshTransform)) false false))))
    (else
      (Variables|Default|SetisHolding false))))

(fn HoverResult
  (if (> (.x (Variables|/Script/Engine.SceneComponent|GetRelativeLocation (Variables|Default|GetButtonMesh))) (+ (.x (.location (Variables|Mesh|GetMeshTransform))) (* (Variables|Mesh|GetArrowHover) 0.8)))
    (Default|TriggerAction (Variables|Blueprints|GetShip) (Variables|Function|GetAction))))